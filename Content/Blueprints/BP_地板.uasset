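; Editor-time floor generator that fills an area sized by a ruler transform (扩张标尺) in its Construction Script.
; It either builds one solid scaled slab or lays a capped grid, spaced by mesh bounds and gaps, under an optional preview slab.
; Seeded streams randomize each tile's mesh, offset, yaw and scale.
; With 设置模型 off, billboards replace tiles; event graph is unused.
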(fn `UserConstructionScript`
  (bind `_地板模型` (`self.地板模型`))
  (bind `_z轴偏移` (`self.z轴偏移`))
  (bind `_z轴随机偏移` (`self.z轴随机偏移`))
  (bind `_变换随机种` (`self.变换随机种`))
  (bind `_变换随机种_2` (`self.变换随机种`))
  (bind `_扩张标尺_location` (`KismetMathLibrary.BreakTransform` (`self.扩张标尺`)))
  (bind `_扩张标尺` (`self.扩张标尺`))
  (bind `_扩张标尺_2` (`self.扩张标尺`))
  (bind `_缩放尺寸` (`self.缩放尺寸`))
  (bind `_旋转角度` (`self.旋转角度`))
  (bind `_旋转随机角度` (`self.旋转随机角度`))
  (bind `_变换随机偏移` (`self.变换随机偏移`))
  (bind _returnvalue (/ `_扩张标尺_location` 100))
  (bind _returnvalue_2 (* `_扩张标尺_location` (0.0 0.5 0.0)))
  (bind _returnvalue_3 (* (`self.缩放随机尺寸`) 0.01))
  (bind _returnvalue_4 (`KismetMathLibrary.RandomFloatInRangeFromStream` (- `_旋转角度` `_旋转随机角度`) (+ `_旋转角度` `_旋转随机角度`) `_变换随机种`))
  (bind _returnvalue_5 (`KismetMathLibrary.RandomFloatInRangeFromStream` (* -1 `_变换随机偏移`) `_变换随机偏移` `_变换随机种_2`))
  (bind _returnvalue_6 (`KismetMathLibrary.Conv_IntToDouble` (- (`self.最大生成`) 1)))
  (bind _returnvalue_7 (`KismetMathLibrary.Conv_DoubleToVector` (`KismetMathLibrary.RandomFloatInRangeFromStream` (- `_缩放尺寸` _returnvalue_3) (+ `_缩放尺寸` _returnvalue_3) `_变换随机种`)))
  (bind _output (`|GetArrayItem` `_地板模型` (`KismetMathLibrary.RandomIntegerInRangeFromStream` 0 (- (`KismetArrayLibrary.Array_Length` `_地板模型`) 1) (`self.模型随机种`))))
  (bind _returnvalue_8 (`StaticMesh.GetBounds` _output))
  (bind _returnvalue_9 (+ (* 2 (.y (`.BoxExtent` (`KismetMathLibrary.BreakBoxSphereBounds` _returnvalue_8)))) (`self.Y轴间隔`)))
  (bind _returnvalue_10 (+ (* 2 (.x (`.BoxExtent` (`KismetMathLibrary.BreakBoxSphereBounds` _returnvalue_8)))) (`self.X轴间隔`)))
  (bind _returnvalue_11 (/ (.x (.location `_扩张标尺_2`)) _returnvalue_10))
  (bind _returnvalue_12 (/ (.y (.location `_扩张标尺_2`)) _returnvalue_9))
  (if (`self.实体化绿片模型`)
    (bind _returnvalue_13 (`AddComponent|NODE_AddStaticMeshComponent-4` :`RelativeTransform` (`KismetMathLibrary.MakeTransform` _returnvalue_2 (struct) _returnvalue)))
    (`PrimitiveComponent.SetMaterial` _returnvalue_13 0 (`self.材质`))
    (else
      (if (not (`self.隐藏绿片`))
        (`AddComponent|NODE_AddStaticMeshComponent-3` :`RelativeTransform` (`KismetMathLibrary.MakeTransform` (+ _returnvalue_2 (0.0 0.0 5.0)) (struct) _returnvalue)))
      (bind _returnvalue_14 (`AddComponent|NODE_AddBillboardComponent-2` :`RelativeTransform` (`KismetMathLibrary.MakeTransform` (`KismetMathLibrary.MakeVector` (.x (.location `_扩张标尺`)) (.y (.location `_扩张标尺`)) (.z (`.BoxExtent` (`KismetMathLibrary.BreakBoxSphereBounds` _returnvalue_8)))) (.rotation `_扩张标尺`) (* (.scale `_扩张标尺`) (`self.标尺尺寸`)))))
      (`SceneComponent.SetVisibility` _returnvalue_14 (`self.显示UI`) false)
      (for _index (range (+ (`KismetMathLibrary.Abs_Int` (`KismetMathLibrary.FTrunc` (`KismetMathLibrary.FMin` (- _returnvalue_11 1.0) _returnvalue_6))) 1))
        (for _index_2 (range (+ (`KismetMathLibrary.Abs_Int` (`KismetMathLibrary.FTrunc` (`KismetMathLibrary.FMin` _returnvalue_6 (- _returnvalue_12 1.0)))) 1))
          (set `self.模型ID` (* _index_2 _index))
          (if (`self.设置模型`)
            (bind _returnvalue_15 (+ (`KismetMathLibrary.MakeVector` (* (`KismetMathLibrary.FTrunc` (`KismetMathLibrary.SignOfFloat` _returnvalue_11)) (* _index _returnvalue_10)) (* (`KismetMathLibrary.FTrunc` (`KismetMathLibrary.SignOfFloat` _returnvalue_12)) (* _index_2 _returnvalue_9))) (`KismetMathLibrary.MakeVector` _returnvalue_5 _returnvalue_5 (`KismetMathLibrary.RandomFloatInRangeFromStream` (- `_z轴偏移` `_z轴随机偏移`) (+ `_z轴偏移` `_z轴随机偏移`) `_变换随机种_2`))))
            (bind _returnvalue_16 (`AddComponent|NODE_AddStaticMeshComponent-2` :`RelativeTransform` (`KismetMathLibrary.MakeTransform` _returnvalue_15 (`KismetMathLibrary.MakeRotator` 0.0 0.0 _returnvalue_4) _returnvalue_7)))
            (`PrimitiveComponent.SetMaterial` _returnvalue_16 0 (`self.地板材质设置`))
            (`StaticMeshComponent.SetStaticMesh` _returnvalue_16 _output)
            (else
              (bind _returnvalue_17 (`AddComponent|NODE_AddBillboardComponent-1` :`RelativeTransform` (`KismetMathLibrary.MakeTransform` (+ _returnvalue_15 (0.0 0.0 50.0)) (`KismetMathLibrary.MakeRotator` 0.0 0.0 _returnvalue_4) _returnvalue_7)))
              (`SceneComponent.SetVisibility` _returnvalue_17 (`self.显示UI`) false))))))))