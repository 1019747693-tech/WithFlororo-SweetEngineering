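; Visual layer of the turn-based tactics grid, drawing tiles through two instanced-mesh actors: a flat grid and a tactical view.
; Tile updates refresh both; tactical tiles stretch down to the lowest recorded height.
; Tactical regeneration is deferred while that view is hidden; toggling it also hides or shows NotTactical-tagged actors.
; In game, the child actors are replaced by spawned actors to work around UE 5.4 instability.
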(event `self.ReceiveBeginPlay`
  (`self.SetActorTickEnabled` false))

(fn `Destroy Grid Visual`
  (bind _gridmeshinst_tactical (`self.GridMeshInst_Tactical`))
  (bind _gridmeshinst (`self.GridMeshInst`))
  ;[0 0 0] [EN] Clear instances on components
  ; [FR] Détruit les instances des components
  ; [CN] 清除组件上的实例
  (`|ExecutionSequence`
    (:`then_0`
      (`/Engine/EditorBlueprintResources/StandardMacros.IsValid` _gridmeshinst
        (:`Is Valid`
          (`/Game/TurnBasedTactic/Blueprints/Core/Grid/Utilities/BP_GridMeshInst.ClearInstances` _gridmeshinst))))
    (:`then_1`
      (`/Engine/EditorBlueprintResources/StandardMacros.IsValid` _gridmeshinst_tactical
        (:`Is Valid`
          (`/Game/TurnBasedTactic/Blueprints/Core/Grid/Utilities/BP_GridMeshInst.ClearInstances` _gridmeshinst_tactical))))
    (:`then_2`
      (`self.Set Grid Lowest Z` 999999.0))))

(fn `Initialize Grid Visual`
  (params (Grid :type "/Game/TurnBasedTactic/Blueprints/Core/Grid/BP_Grid Object Reference"))
  (bind (_meshsize _mesh _meshmaterial) (break `/Game/TurnBasedTactic/Blueprints/Core/Grid/GridShapes/S_GridShapeData` (`/Game/TurnBasedTactic/Blueprints/Core/Grid/BP_Grid.GetCurrentShapeData` (`self.Grid`))))
  (bind (_meshsize_2 _mesh_2 _meshmaterial_2 _flatmesh _flatmaterial) (break `/Game/TurnBasedTactic/Blueprints/Core/Grid/GridShapes/S_GridShapeData` (`/Game/TurnBasedTactic/Blueprints/Core/Grid/BP_Grid.GetCurrentShapeData` (`self.Grid`))))
  ;[0 0 0] [EN] Setup the references
  ; [FR] Initialise les références
  ; [CN] 初始化引用
  (set `self.Grid` Grid)
  (bind (_grid _tactical) (`self.UE 5 4 0 Bug Replace Child Actors With Real Actors`))
  (set `self.GridMeshInst` _grid)
  (set `self.GridMeshInst_Tactical` _tactical)
  ;[0 0 0] [EN] Setup the components
  ; [FR] Initialise les components
  ; [CN] 初始化组件
  (`/Game/TurnBasedTactic/Blueprints/Core/Grid/Utilities/BP_GridMeshInst.Initialize Grid Mesh Inst` (`self.GridMeshInst`) _flatmesh _flatmaterial false "QueryOnly")
  (`/Game/TurnBasedTactic/Blueprints/Core/Grid/Utilities/BP_GridMeshInst.Initialize Grid Mesh Inst` (`self.GridMeshInst_Tactical`) _mesh _meshmaterial true "QueryOnly")
  ;[0 0 0] [EN] Center grid in world
  ; [FR] Centre la gille dans le monde
  ; [CN] 将网格居中于世界坐标系
  (`self.K2_SetActorLocation` (0.0 0.0 0.0)) ; Center actor in world
  ;[0 0 0] [EN] Set grid's height
  ; [FR] Applique la hauteur de la grille
  ; [CN] 设置网格高度
  (`self.Set Offset from Ground` (`self.OffsetFromGround`))
  ;[0 0 0] [EN] Reset height of the grid
  ; [FR] Reset la hauteur de la grille
  ; [CN] 重置网格高度
  (`self.Set Grid Lowest Z` 999999.0)
  ;[0 0 0] [EN] Apply the default IsTactical
  ; [FR] Applique le defaut IsTactical
  ; [CN] 应用默认的IsTactical设置
  (`self.Set Is Tactical` (`self.IsTactical`)))

(fn `Set Grid Lowest Z`
  (params (Z :type "Float (double-precision)" :default 999999.0))
  (set `self.GridLowestZ` Z)
  (set `self.NeedToReGenerateTacticalOnNextEnable` true))

(fn `Set Is Tactical`
  (params (Tactical :type Boolean))
  (bind _gridmeshinst_tactical (`self.GridMeshInst_Tactical`))
  (bind _grid (`self.Grid`))
  (set `self.IsTactical` Tactical)
  ;[0 0 0] [EN] If tactical is enabled, we show the grid and hide all the NotTactical actors. And vice-versa.
  ; [FR] Si le mode tactique est activé, on montre la grille et on cache tous les actors NotTactical. Et vice-versa
  ; [CN] 若启用战术模式，则显示网格并隐藏所有非战术角色，反之亦然。
  (`self.SetActorHiddenInGame` (`self.GridMeshInst_Tactical`) (not (`self.IsTactical`)))
  (bind _outactors (`GameplayStatics.GetAllActorsWithTag` "NotTactical"))
  (for _array_element _outactors
    (`self.SetActorHiddenInGame` _array_element (`self.IsTactical`)))
  ;[0 0 0] [EN] If tactical is enabled and we needed to regenerate the grid, do it.
  ; [FR] Si le mode tactique est activé et qu'il fallait regénérer la grille, on le fait.
  ; [CN] 若战术模式已启用且需重新生成网格，则执行生成操作。
  (`|ExecutionSequence`
    (:`then_0`
      (if (and (`self.IsTactical`) (`self.NeedToReGenerateTacticalOnNextEnable`))
        (set `self.NeedToReGenerateTacticalOnNextEnable` false)
        (`/Engine/EditorBlueprintResources/StandardMacros.IsValid` _grid ; Invalid if grid never generated\n若网格从未生成则无效
          (:`Is Valid`
            (bind _values (`BlueprintMapLibrary.Map_Values` (`/Game/TurnBasedTactic/Blueprints/Core/Grid/BP_Grid.GridTiles` _grid)))
            (for _array_element_2 _values
              (`self.Update Tile Visual Tactical` _array_element_2))))))
    (:`then_1`
      (`/Engine/EditorBlueprintResources/StandardMacros.IsValid` _gridmeshinst_tactical ; Invalid if grid never generated\n若网格从未生成则无效
        (:`Is Valid`
          (`PrimitiveComponent.SetCollisionEnabled` (`/Game/TurnBasedTactic/Blueprints/Core/Grid/Utilities/BP_GridMeshInst.InstancedStaticMesh` _gridmeshinst_tactical) (select `bool` (`self.IsTactical`) :`false` "NoCollision" :`true` "QueryOnly" :!type "ECollisionEnabled Enum")))))))

(fn `Set Offset from Ground`
  (params (Offset :type "Float (double-precision)"))
  ;[0 0 0] [EN] Set grid's height, do not touch the X and Y
  ; [FR] Applique la hauteur de la grille, ne touche pas le X et Y
  ; [CN] 设置网格高度，保持X和Y轴不变
  (set `self.OffsetFromGround` Offset)
  (`self.K2_SetActorRelativeLocation` (`self.GridMeshInst`) (`KismetMathLibrary.MakeVector` 0.0 0.0 (`self.OffsetFromGround`)) false false))

(fn `UE 5 4 0 Bug Replace Child Actors With Real Actors`
  (returns (Grid :type "/Game/TurnBasedTactic/Blueprints/Core/Grid/Utilities/BP_GridMeshInst Object Reference") (Tactical :type "/Game/TurnBasedTactic/Blueprints/Core/Grid/Utilities/BP_GridMeshInst Object Reference"))
  (locals (SpawnedGrid :type "/Game/TurnBasedTactic/Blueprints/Core/Grid/Utilities/BP_GridMeshInst Object Reference") (SpawnedTactical :type "/Game/TurnBasedTactic/Blueprints/Core/Grid/Utilities/BP_GridMeshInst Object Reference"))
  (if (`/Game/TurnBasedTactic/Blueprints/Core/Utilities/BFL_Utilities.IsInGame`)
    (`/Engine/EditorBlueprintResources/StandardMacros.IsValid` (`self.ChildActor_GridMeshInst`) ; If not valid, already destroyed
      (:`Is Valid`
        (`|ExecutionSequence`
          (:`then_0`
            (bind _returnvalue (`|SpawnActorFromClass` "/Game/TurnBasedTactic/Blueprints/Core/Grid/Utilities/BP_GridMeshInst.BP_GridMeshInst_C" (`KismetMathLibrary.MakeTransform` (0.0 0.0 0.0)) "Undefined" "MultiplyWithRoot" null null))
            (bind _output_get (set `local.SpawnedGrid` _returnvalue))
            (`self.K2_AttachToComponent` _output_get (`self.Scene`) "None" "SnapToTarget" "SnapToTarget" "SnapToTarget" true)
            (`ActorComponent.K2_DestroyComponent` (`self.ChildActor_GridMeshInst`)))
          (:`then_1`
            (bind _returnvalue_2 (`|SpawnActorFromClass` "/Game/TurnBasedTactic/Blueprints/Core/Grid/Utilities/BP_GridMeshInst.BP_GridMeshInst_C" (`KismetMathLibrary.MakeTransform` (0.0 0.0 0.0)) "Undefined" "MultiplyWithRoot" null null))
            (bind _output_get_2 (set `local.SpawnedTactical` _returnvalue_2))
            (`self.K2_AttachToComponent` _output_get_2 (`self.Scene`) "None" "SnapToTarget" "SnapToTarget" "SnapToTarget" true)
            (`ActorComponent.K2_DestroyComponent` (`self.ChildActor_GridMeshInst_Tactical`)))
          (:`then_2`
            (`KismetSystemLibrary.PrintString` "Warning - Due to instabilities with Child Actors (5.4 and up), ChildActor_GridMeshInst and ChildActor_GridMeshInst_Tactical have been destroyed and replaced by normal actors spawned at runtime." true true (struct :`R` 1.0 :`G` 0.472817 :`A` 1.0) 1.0)
            (return (`local.SpawnedGrid`) (`local.SpawnedTactical`)))))
      (:`Is Not Valid`
        (return (`self.GridMeshInst`) (`self.GridMeshInst_Tactical`))))
    (else
      (return (cast `/Game/TurnBasedTactic/Blueprints/Core/Grid/Utilities/BP_GridMeshInst` (`ChildActorComponent.ChildActor` (`self.ChildActor_GridMeshInst`)) :!pure true) (cast `/Game/TurnBasedTactic/Blueprints/Core/Grid/Utilities/BP_GridMeshInst` (`ChildActorComponent.ChildActor` (`self.ChildActor_GridMeshInst_Tactical`)) :!pure true)))))

(fn `Update Tile Visual`
  (params (Data :type "/Game/TurnBasedTactic/Blueprints/Core/Grid/Utilities/S_TileData Structure"))
  (bind ((`Index_2_FAF085314405A9912C6A66BF3F3BBCCD` _index) (`Type_5_7348A67046FF7B2ACB404DA293B43DAF` _type)) (break `/Game/TurnBasedTactic/Blueprints/Core/Grid/Utilities/S_TileData` (`local.Data`)))
  (bind ((`Index_2_FAF085314405A9912C6A66BF3F3BBCCD` _index_2) (`Type_5_7348A67046FF7B2ACB404DA293B43DAF` _type_2) (`Transform_8_93233B1349F988EACD845197CA733B58` _transform) (`States_12_430F0B8949705184C373EAA0148089ED` _states)) (break `/Game/TurnBasedTactic/Blueprints/Core/Grid/Utilities/S_TileData` (`local.Data`)))
  ;[0 0 0] [EN] Update tile visual based on its data
  ; [FR] Met a jour le visuel de la case basé sur son data
  ; [CN] 根据数据更新格子视觉效果
  (`|ExecutionSequence`
    (:`then_0`
      (`/Game/TurnBasedTactic/Blueprints/Core/Grid/Utilities/BP_GridMeshInst.Remove Instance` (`self.GridMeshInst`) _index)
      (if (`/Game/TurnBasedTactic/Blueprints/Core/Grid/Utilities/BFL_TileData.Is Tile Type Walkable` _type)
        (`/Game/TurnBasedTactic/Blueprints/Core/Grid/Utilities/BP_GridMeshInst.AddInstance` (`self.GridMeshInst`) _index_2 _type_2 _transform _states)))
    (:`then_1`
      (`self.Update Tile Visual Tactical` Data))))

(fn `Update Tile Visual Tactical`
  (params (Data :type "/Game/TurnBasedTactic/Blueprints/Core/Grid/Utilities/S_TileData Structure"))
  (bind ((`Index_2_FAF085314405A9912C6A66BF3F3BBCCD` _index) (`Type_5_7348A67046FF7B2ACB404DA293B43DAF` _type) (`Transform_8_93233B1349F988EACD845197CA733B58` _transform)) (break `/Game/TurnBasedTactic/Blueprints/Core/Grid/Utilities/S_TileData` (`local.Data`)))
  (bind ((`Index_2_FAF085314405A9912C6A66BF3F3BBCCD` _index_2) (`Type_5_7348A67046FF7B2ACB404DA293B43DAF` _type_2) (`Transform_8_93233B1349F988EACD845197CA733B58` _transform_2) (`States_12_430F0B8949705184C373EAA0148089ED` _states)) (break `/Game/TurnBasedTactic/Blueprints/Core/Grid/Utilities/S_TileData` (`local.Data`)))
  (bind _z (.z (`.MeshSize_2_9D2C96BF4606BD546B18CD8906A89D0A` (break `/Game/TurnBasedTactic/Blueprints/Core/Grid/GridShapes/S_GridShapeData` (`/Game/TurnBasedTactic/Blueprints/Core/Grid/BP_Grid.GetCurrentShapeData` (`self.Grid`))))))
  (`|ExecutionSequence`
    (:`then_0`
      ;[0 0 0] [EN] Check if this tile is now the lowest tile on the grid
      ; [FR] Regarde si la case actuelle est maintenant la case la plus basse de la grille
      ; [CN] 检查当前格子是否已成为网格中最低的格子
      (if (< (.z (.location (`.Transform_8_93233B1349F988EACD845197CA733B58` (break `/Game/TurnBasedTactic/Blueprints/Core/Grid/Utilities/S_TileData` (`local.Data`))))) (`self.GridLowestZ`))
        (`self.Set Grid Lowest Z` (.z (.location (`.Transform_8_93233B1349F988EACD845197CA733B58` (break `/Game/TurnBasedTactic/Blueprints/Core/Grid/Utilities/S_TileData` (`local.Data`))))))))
    (:`then_1`
      ;[0 0 0] [EN] Don't calculate everything if the tactical grid is hidden
      ; [FR] Ne calcul pas tout si la grille tactique est cachée
      ; [CN] 若战术网格已隐藏则无需计算所有内容
      (if (`self.IsTactical`)
        ;[0 0 0] [EN] Update tile's visual and make sure to stretch it all the way to the ground
        ; [FR] Met à jour le visuel de la case et fait sûr de l'étirée jusqu'au sol
        ; [CN] 更新格子视觉效果并确保其始终延伸至地面
        (`/Game/TurnBasedTactic/Blueprints/Core/Grid/Utilities/BP_GridMeshInst.Remove Instance` (`self.GridMeshInst_Tactical`) _index)
        (if (`|EnumInequality` _type "NewEnumerator0")
          (`/Game/TurnBasedTactic/Blueprints/Core/Grid/Utilities/BP_GridMeshInst.AddInstance` (`self.GridMeshInst_Tactical`) _index_2 _type_2 (`KismetMathLibrary.MakeTransform` (.location _transform_2) (.rotation _transform_2) (`KismetMathLibrary.MakeVector` (.x (.scale _transform_2)) (.y (.scale _transform_2)) (/ (+ (- (.z (.location _transform)) (`self.GridLowestZ`)) _z) _z))) _states))
        (else
          (set `self.NeedToReGenerateTacticalOnNextEnable` true))))))

(fn `UserConstructionScript`)