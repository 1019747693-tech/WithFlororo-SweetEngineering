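; BP_GridMeshInst is a grid display actor that renders tiles as instances of one InstancedStaticMesh, with configurable mesh, material and collision.
; InstanceIndexes maps grid indices to instances, and adding a tile first removes any existing one at that index.
; Four per-instance custom data floats carry a fill flag and RGB, colored by tile type or by the highest-priority tile state.
; The component's NumCustomDataFloat must be 4.
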(event `self.ReceiveBeginPlay`
  (`self.SetActorTickEnabled` false))

(fn `AddInstance`
  (params (Index :type "IntPoint Structure (by ref)") (TileType :type "/Game/TurnBasedTactic/Blueprints/Core/Grid/Utilities/E_TileType Enum" :default "NewEnumerator0") (Transform :type "Transform Structure (by ref)") (States :type "Array of /Game/TurnBasedTactic/Blueprints/Core/Grid/Utilities/E_TileState Enum"))
  (locals (I :type Integer))
  (bind _instancedstaticmesh (`self.InstancedStaticMesh`))
  (bind _i (`local.I`))
  ;[0 0 0] [EN] Remove instance first because we can only have one tile per index. Then update the transform and add it to the array for future access.
  ; [FR] Premièrement, il faut enlever l'instance parce qu'on peut en avoir qu'une par index. Puis on met a jour le transform et on l'ajoute a une liste pour pouvoir y accéder plus tard
  ; [CN] 首先移除实例（每个索引仅允许存在一个格子），随后更新变换并将其添加至数组以供后续访问。
  (`self.Remove Instance` Index)
  (`InstancedStaticMeshComponent.AddInstance` (`self.InstancedStaticMesh`) Transform false)
  (bind _returnvalue (`KismetArrayLibrary.Array_Add` (`self.InstanceIndexes`) Index))
  (set `local.I` _returnvalue)
  ;[0 0 0] [EN] Use CusomDataValue to set the colors to the specific tiles we want
  ; -  IMPORTANT!   -  Make sure to set the NumCustomDataFloat to 4 in the Component
  ;
  ; [FR] Utiliser les CustomDataValue pour changer la couleur des cases que nous voulons
  ; -  IMPORTANT!   -  Mettez le NumCustomDataFloat à 4 dans le Component
  ;
  ; 0 = IsFilled   |   1 = R   |   2 = G   |   3 = B
  ; [CN] 使用CustomDataValue为指定格子设置颜色
  ; - 重要！确保在组件中将NumCustomDataFloat设置为4
  ;
  ; 0 = 是否填充 | 1 = 红 | 2 = 绿 | 3 = 蓝
  (bind (_isfilled _color) (`self.Get Color from States or Type` (`local.TileType`) (`local.States`)))
  (`InstancedStaticMeshComponent.SetCustomDataValue` _instancedstaticmesh _i 0 _isfilled false) ; 0 = IsFilled
  (bind (_r _g _b) (`KismetMathLibrary.BreakColor` _color))
  (`InstancedStaticMeshComponent.SetCustomDataValue` _instancedstaticmesh _i 1 _r false) ; 1 = R
  (`InstancedStaticMeshComponent.SetCustomDataValue` _instancedstaticmesh _i 2 _g false) ; 2 = G
  (`InstancedStaticMeshComponent.SetCustomDataValue` _instancedstaticmesh _i 3 _b false) ; 3 = B
)

(fn `ClearInstances`
  ;[0 0 0] [EN] Delete all instances and clear the array
  ; [FR] Supprime toutes les instances et vide la liste
  ; [CN] 删除所有实例并清空数组
  (`InstancedStaticMeshComponent.ClearInstances` (`self.InstancedStaticMesh`))
  (`KismetArrayLibrary.Array_Clear` (`self.InstanceIndexes`)))

(fn `Get Color from States or Type`
  (params (TileType :type "/Game/TurnBasedTactic/Blueprints/Core/Grid/Utilities/E_TileType Enum" :default "NewEnumerator0") (States :type "Array of /Game/TurnBasedTactic/Blueprints/Core/Grid/Utilities/E_TileState Enum"))
  (returns (IsFilled :type "Float (double-precision)") (Color :type "LinearColor Structure"))
  (if (`self.IsColorBasedOnTileType`)
    (return 1.0 (`/Game/TurnBasedTactic/Blueprints/Core/Grid/Utilities/BFL_TileData.Get Tile Type Color` (`local.TileType`)))
    (else
      ;[0 0 0] [EN] Based on the Tile States, return the first color we find in our Priority List
      ; [FR] Basé sur les States de notre tile, retourne la première couleur que nous trouvons dans notre Priority List
      ; [CN] 根据格子状态，按优先级列表返回首个匹配的颜色
      (if (== (`KismetArrayLibrary.Array_Length` States) 0)
        (return 0.0)
        (else
          (for _array_element (`/Game/TurnBasedTactic/Blueprints/Core/Grid/Utilities/BFL_TileData.Get Sorted List Of Tile States`)
            (if (`KismetArrayLibrary.Array_Contains` (`local.States`) _array_element)
              (return 1.0 (`/Game/TurnBasedTactic/Blueprints/Core/Grid/Utilities/BFL_TileData.GetTileStateColor` _array_element))))
          (return 0.0))))))

(fn `Initialize Grid Mesh Inst`
  (params (Mesh :type "StaticMesh Object Reference") (Material :type "MaterialInterface Object Reference") (ColorBasedOnTileType :type Boolean) (Collision :type "ECollisionEnabled Enum" :default "NoCollision"))
  (bind _instancedstaticmesh (`self.InstancedStaticMesh`))
  ;[0 0 0] [EN] Sets the default data needed to display this grid
  ; [FR] Applique les valeurs par défaut que l'acteur à besoin pour afficher la grille
  ; [CN] 设置显示此网格所需的默认数据
  (`StaticMeshComponent.SetStaticMesh` _instancedstaticmesh Mesh)
  (`PrimitiveComponent.SetMaterial` _instancedstaticmesh 0 Material)
  (set `self.IsColorBasedOnTileType` ColorBasedOnTileType)
  (`PrimitiveComponent.SetCollisionEnabled` _instancedstaticmesh Collision))

(fn `Remove Instance`
  (params (Index :type "IntPoint Structure (by ref)"))
  (bind _instanceindexes (`self.InstanceIndexes`))
  ;[0 0 0] [EN] Remove instance and remove it from the array
  ; [FR] Enlève l'instance et la retire de la liste
  ; [CN] 移除实例并将其从数组中删除
  (if (`KismetArrayLibrary.Array_Contains` _instanceindexes Index)
    (`InstancedStaticMeshComponent.RemoveInstance` (`self.InstancedStaticMesh`) (`KismetArrayLibrary.Array_Find` _instanceindexes Index))
    (`KismetArrayLibrary.Array_RemoveItem` (`self.InstanceIndexes`) Index)))

(fn `UserConstructionScript`)