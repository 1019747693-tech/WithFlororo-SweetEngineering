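; BP_GridModifier is a volume for the tactics grid that marks an area with a tile type such as obstacle, extra movement cost or flying-only.
; The construction script takes mesh and flat material from the Shape data and colors them by Type.
; It then sets collision, since changing the mesh resets it: overlap on the ground trace channel, Pawn blocking only for obstacles.
; The volume is hidden in game and has no runtime logic.
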(fn `UserConstructionScript`
  (bind _staticmesh (`self.StaticMesh`))
  (bind _staticmesh_2 (`self.StaticMesh`))
  (bind ((`Mesh_5_762547C8443C5216D6D0F89D90BAB1D7` _mesh) (`FlatMaterial_18_4DFF26A0455E97246F7C91BCAA82703D` _flatmaterial)) (break `/Game/TurnBasedTactic/Blueprints/Core/Grid/GridShapes/S_GridShapeData` (`/Game/TurnBasedTactic/Blueprints/Core/Grid/GridShapes/BFL_GridShape.GetShapeData` (`self.Shape`))))
  ;[0 0 0] [EN] Set volume's visual based on the shape and type
  ; [FR] Set le visuel de notre volume basé sur la shape et le type
  ; [CN]根据形状和类型设置体积的视觉效果
  (`StaticMeshComponent.SetStaticMesh` _staticmesh_2 _mesh)
  (`PrimitiveComponent.SetMaterial` _staticmesh_2 0 _flatmaterial)
  (`MeshComponent.SetVectorParameterValueOnMaterials` _staticmesh_2 "Color" (`KismetMathLibrary.Conv_LinearColorToVector` (select `/Game/TurnBasedTactic/Blueprints/Core/Grid/Utilities/E_TileType` (`self.Type`) :`NewEnumerator1` (struct :`R` 1.0 :`G` 1.0 :`B` 1.0 :`A` 1.0) :`NewEnumerator2` (struct :`R` 0.682292 :`G` 0.053304 :`B` 0.053304 :`A` 1.0) :`NewEnumerator3` (struct :`R` 0.729412 :`G` 0.298039 :`B` 0.082353 :`A` 1.0) :`NewEnumerator4` (struct :`R` 0.32549 :`G` 0.137255 :`A` 1.0) :`NewEnumerator5` (struct :`R` 0.533333 :`G` 0.286275 :`B` 0.560784 :`A` 1.0) :!type "LinearColor Structure")))
  (`MeshComponent.SetScalarParameterValueOnMaterials` _staticmesh_2 "IsFilled" 1.0)
  ;[0 0 0] [EN] The volume should overlap the same trace channel as the ground. We have to set it after setting the mesh, because the SetStaticMesh function resets this setting
  ; [FR] Le volume doit overlap le même trace channel que le ground. On doit le set après avoir set le mesh parce la fonction SetStaticMesh reset ce paramètre.
  ; [CN]该体积应与地面使用相同的追踪通道（或 “该体积的追踪通道应与地面重叠”）。我们必须在设置网格体之后再进行此项设置，因为 SetStaticMesh（设置静态网格体）函数会重置该配置。
  (`PrimitiveComponent.SetCollisionResponseToChannel` _staticmesh "ECC_GameTraceChannel1" "ECR_Overlap")
  (`PrimitiveComponent.SetCollisionResponseToChannel` _staticmesh "ECC_GameTraceChannel4" "ECR_Block")
  (`PrimitiveComponent.SetCollisionResponseToChannel` _staticmesh "ECC_Pawn" (select `bool` (`|EnumEquality` (`self.Type`) "NewEnumerator2") :`false` "ECR_Ignore" :`true` "ECR_Block" :!type "ECollisionResponse Enum"))
  ;[0 0 0] [EN] Don't want to see this volume in game
  ; [FR] On ne veut pas voir ce volume dans le jeu
  ; [CN]游戏运行后隐藏体积
  (`self.SetActorHiddenInGame` true))