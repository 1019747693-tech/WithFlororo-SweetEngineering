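; Spell animation that calls in or redirects the casting unit's aircraft at the targeted grid tile in turn-based tactical combat.
; It searches for an existing aircraft manager by a tag built from unit, spell animation and aircraft names, spawning one at the tile if none exists.
; An existing manager is retargeted by tile occupant: self, ally escort, enemy attack, or air patrol when empty.
; The animation completes immediately after issuing the order.
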(event `self.Event_PlaySpellAnimation`
  (set `self.Target_Index` (`|GetArrayItem` (`/Game/TurnBasedTactic/Blueprints/Core/Combat/BP_CombatSystem.AttackedIndex` (`self.CombatSystem`))))
  (bind _outactors (`GameplayStatics.GetAllActorsWithTag` (`KismetStringLibrary.Conv_StringToName` (`KismetStringLibrary.Concat_StrStr` (`KismetSystemLibrary.GetObjectName` (`self.Unit`)) "_" (`self.SA_Name`) "_" (`KismetStringLibrary.Conv_NameToString` (`.Attack_Unit_Name_7_BECA54CF461C14C6D44E1E814BE2B8BE` (break `/Game/TurnBasedTactic/Blueprints/Core/Combat/Spells/SpellAnimations/Material/SA_Attack_Interactive/Materical/E_ATI_Assets` (`.Attack_Interactive_Asset_3_BECA54CF461C14C6D44E1E814BE2B8BE` (break `/Game/TurnBasedTactic/Blueprints/Core/Combat/Spells/SpellAnimations/Material/SA_Attack_Interactive/Materical/E0_ATI_Date` (`.ATI_Date` (defaults `Object` (`self.Aircraft_Manager`))))))))))))
  (if (> (`KismetArrayLibrary.Array_Length` _outactors) 0)
    (`KismetSystemLibrary.PrintText` "已检测到自己名下ACM,不进行生成")
    (bind (_eaircraftstate _target_unit) (`self.F_Get_Grid_Switch_ACM_State`))
    (bind _output_get (set `self.SA_ACM` (cast `/Game/TurnBasedTactic/Blueprints/Core/Combat/Spells/SpellAnimations/Material/SA_Attack_Interactive/Aircraft_Manager/BP_Aircraft_Manager` (`|GetArrayItem` _outactors) :!pure true)))
    (`/Game/TurnBasedTactic/Blueprints/Core/Combat/Spells/SpellAnimations/Material/SA_Attack_Interactive/Aircraft_Manager/BP_Aircraft_Manager.Change_Target` _output_get _eaircraftstate (`self.Target_Index`) _target_unit)
    (else
      (`KismetSystemLibrary.PrintText` "未搜索到自己名下ACM,进行创建")
      (`self.Brith_Manager`)))
  (`self.Event_CompleteSpellAnimation`))

(event `Brith_Manager`
  (bind _unit (`self.Unit`))
  ;[1 1 1] 在不存在自己名下SA,ACM的情况下,创建ACM的飞机
  (bind _returnvalue (`|SpawnActorFromClass` (`self.Aircraft_Manager`) (`KismetMathLibrary.MakeTransform` (`/Game/TurnBasedTactic/Blueprints/Core/Grid/BP_Grid.GetTileLocationFromGridIndex` (`self.Grid`) (`self.Target_Index`))) "Undefined" "MultiplyWithRoot" null (`/Game/TurnBasedTactic/Blueprints/Core/Units/0_BP_Unit.TeamIndex` _unit) _unit self null))
  (`/Game/TurnBasedTactic/Blueprints/Core/Combat/Spells/SpellAnimations/Material/SA_Attack_Interactive/Aircraft_Manager/BP_Aircraft_Manager.Birth Aircraft` _returnvalue))

(event `Make_Manager`
  (params (EAircraftState :type "/Game/TurnBasedTactic/Blueprints/Core/Combat/Spells/SpellAnimations/Material/SA_Attack_Interactive/Aircraft_Manager/Materical/EAircraftState Enum" :default "NewEnumerator5") (`Target Unit` :type "/Game/TurnBasedTactic/Blueprints/Core/Units/0_BP_Unit Object Reference"))
  (`/Game/TurnBasedTactic/Blueprints/Core/Combat/Spells/SpellAnimations/Material/SA_Attack_Interactive/Aircraft_Manager/BP_Aircraft_Manager.Change_Target` (`self.SA_ACM`) EAircraftState (`self.Target_Index`) `Target Unit`)
  (`KismetSystemLibrary.PrintText` "SA执行Make_Manager命令"))

(fn `F_Get_Grid_Switch_ACM_State`
  (returns (EAircraftState :type "/Game/TurnBasedTactic/Blueprints/Core/Combat/Spells/SpellAnimations/Material/SA_Attack_Interactive/Aircraft_Manager/Materical/EAircraftState Enum") (Target_Unit :type "/Game/TurnBasedTactic/Blueprints/Core/Units/0_BP_Unit Object Reference"))
  (bind (_target_unit _has_unit_ _teamindex) (`/Game/TurnBasedTactic/Blueprints/Core/Combat/BP_CombatSystem.F Index Find Unit` (`self.CombatSystem`)))
  (if _has_unit_
    (if (== _teamindex (`/Game/TurnBasedTactic/Blueprints/Core/Units/0_BP_Unit.TeamIndex` (`self.Unit`)))
      (`KismetSystemLibrary.PrintText` "护卫")
      (if (== _target_unit (`self.Unit`))
        (return "NewEnumerator0" _target_unit)
        (else
          (return "NewEnumerator1" _target_unit)))
      (else
        (`KismetSystemLibrary.PrintText` "袭击")
        (return "NewEnumerator2" _target_unit)))
    (else
      (`KismetSystemLibrary.PrintText` "空中警戒")
      (return "NewEnumerator6" null))))

(fn `UserConstructionScript`
  (`parent.UserConstructionScript`))