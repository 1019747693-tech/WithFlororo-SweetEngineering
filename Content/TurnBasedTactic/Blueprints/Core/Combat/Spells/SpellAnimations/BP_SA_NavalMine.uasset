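; Spell animation for a turn-based tactics game that scatters naval mines over random tiles from CombatSystem's NullAttackedIndexes list.
; A loop draws and removes random indexes, line-traces for existing interactive attack actors, retries when blocked, and otherwise spawns a mine carrying team, unit and animation references.
; Random picks re-roll per node, so the traced and removed tiles can differ.
; Destroy_By_Torpedo counts detonations and completes the animation at HaveNavalMineNumber.
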(event `self.ReceiveBeginPlay`
  (`parent.ReceiveBeginPlay`)
  (set `self.Destroy_NavalMine_Number` 0))

(event `self.Event_PlaySpellAnimation`
  (bind _nullattackedindexes (`/Game/TurnBasedTactic/Blueprints/Core/Combat/BP_CombatSystem.NullAttackedIndexes` (`self.CombatSystem`)))
  (bind _output (`|GetArrayItem` _nullattackedindexes (`KismetMathLibrary.RandomIntegerInRange` 0 (- (`KismetArrayLibrary.Array_Length` _nullattackedindexes) 1))))
  (bind _tilelocation (`/Game/TurnBasedTactic/Blueprints/Core/Grid/BP_Grid.GetTileLocationFromGridIndex` (`self.Grid`) _output))
  (`KismetArrayLibrary.Array_Clear` (`self.Brith_NavalMine_Position`))
  (set `self.Number` (`self.NavalMine_Number`))
  (if (>= (`self.Number`) 0) :!label _label
    (if (<= (`KismetArrayLibrary.Array_Length` (`/Game/TurnBasedTactic/Blueprints/Core/Combat/BP_CombatSystem.NullAttackedIndexes` (`self.CombatSystem`))) 0)
      (`KismetSystemLibrary.PrintText` "初始集合里已空,不再生成" false)
      (else
        (bind (_outhit _returnvalue) (`KismetSystemLibrary.LineTraceSingle` :`Start` (+ (0.0 0.0 1000.0) _tilelocation) :`End` _tilelocation :`TraceChannel` "TraceTypeQuery7" :`DrawDebugType` "ForDuration")) ; 命中ATI,如果命中,判断是否为水雷,会在不是的地方生成.
        (`KismetArrayLibrary.Array_RemoveItem` (`/Game/TurnBasedTactic/Blueprints/Core/Combat/BP_CombatSystem.NullAttackedIndexes` (`self.CombatSystem`)) _output)
        (if _returnvalue
          (if (`.bSuccess` (cast `/Game/TurnBasedTactic/Blueprints/Core/Combat/Spells/SpellAnimations/Material/SA_Attack_Interactive/0_BP_Attack_Interactive_ATI` (`.HitActor` (`GameplayStatics.BreakHitResult` _outhit)) :!pure true))
            (`KismetSystemLibrary.PrintText` "命中已有水雷,重新生成" false false)
            (goto _label)
            (else
              _)))
        (`self.F_Brith_Navalmine` (`.TraceEnd` (`GameplayStatics.BreakHitResult` _outhit)))
        (`/Engine/EditorBlueprintResources/StandardMacros.DecrementInt` (`self.Number`)
          (:`  `
            (goto _label)))))
    (else
      (`KismetSystemLibrary.PrintText` "生成完毕"))))

(event `Destroy_By_Torpedo`
  ;[1 1 1] 计算鱼雷数，到数后销毁自己
  (bind _result (`/Engine/EditorBlueprintResources/StandardMacros.IncrementInt` (`self.Destroy_NavalMine_Number`))
    (:`  `
      (if (== _result (`self.Have_NavalMine_Number`))
        (`KismetSystemLibrary.PrintText` "已被销毁" true false)
        (`self.Event_CompleteSpellAnimation`)
        (else
          (`KismetSystemLibrary.PrintText` (`|FormatText` "{A}发鱼雷已被引爆" _result) true false))))))

(fn `F_Brith_Navalmine`
  (params (Brith_Position :type "Vector Structure"))
  (bind _unit (`self.Unit`))
  (bind _returnvalue (`|SpawnActorFromClass` (`self.NavalMine_Type`) (`KismetMathLibrary.MakeTransform` Brith_Position) "Undefined" "MultiplyWithRoot" null (`/Game/TurnBasedTactic/Blueprints/Core/Units/0_BP_Unit.TeamIndex` _unit) _unit self null))
  (`KismetSystemLibrary.PrintText` "生成一个水雷" false false)
  (`self.K2_DetachFromActor` _returnvalue "KeepRelative" "KeepRelative" "KeepRelative"))

(fn `UserConstructionScript`
  (`parent.UserConstructionScript`))