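; Torpedo attack interactive (ATI) for turn-based tactics: travels forward each move and explodes on enemies or obstacles, ignoring friendlies.
; Construction applies mesh, collision, blast scale and idle VFX from data, plus a child range-icon actor shown on touch.
; When notified, a timeline lerps it forward by speed, then decrements its lifetime and self-destructs at zero.
; Hits stop the timeline and detonate it, also detonating enemy ATIs; a random birth-path actor animates its launch.
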(event `self.ReceiveBeginPlay`
  (`parent.ReceiveBeginPlay`)
  (`self.F_Reset_Materical`))

(event `self.Event_Call_ATI_UnitBegin`
  ;[1 1 1] 通知让鱼雷移动
  (`self.Event_ATI_Move`))

(event `Event_ATI_Move`
  ;[1 0 0] ATI接受母unit通知的事件,
  ; 鱼雷:移动，开始移动后允许引爆
  (set `self.bCanBoom` true)
  (`self.ATI_Move_Torpedo`))

(event `ATI_Move_Torpedo`
  (bind ((`Torpedo_Speed_12_D21B9F8C40718C08D61C7FA65F4A5EA1` _torpedo_speed)) (break `/Game/TurnBasedTactic/Blueprints/Core/Combat/Spells/SpellAnimations/Material/SA_Attack_Interactive/Materical/E_ATI_DateTorpedo` (`self.Torpedo_Date`)))
  (bind _returnvalue (`self.K2_GetActorLocation` self))
  ;[1 0.8136 0 1 36] 鱼雷移动
  (`TimelineComponent.SetPlayRate` (`self.Torpedo_Move`) (/ 1.0 (/ (`KismetMathLibrary.Conv_IntToDouble` _torpedo_speed) 5.0)))
  (set `self.ATI_Begin_position` _returnvalue)
  (set `self.ATI_End_position` (+ _returnvalue (* (`self.GetActorForwardVector` self) (* _torpedo_speed 200))))
  (bind (_direction _torpedo_move) (`Timeline|Torpedo_Move` :!via `PlayFromStart` :!label _label)
    (:`Update`
      (`self.K2_SetActorLocation` self (`KismetMathLibrary.VLerp` (`self.ATI_Begin_position`) (`self.ATI_End_position`) _torpedo_move) false false))
    (:`Finished`
      ;;[1 1 1] 计算剩余回合数，没了之后就自爆
      (bind _result (`/Engine/EditorBlueprintResources/StandardMacros.DecrementInt` (`.Age_Current_15_B1EF7DD84DA60BE5C40CDEBDE7AE72BA` (break `/Game/TurnBasedTactic/Blueprints/Core/Combat/Spells/SpellAnimations/Material/SA_Attack_Interactive/Materical/E_ATI_BaseState` (`.BaseState_9_997CD240407AC492B23DB296C2061696` (break `/Game/TurnBasedTactic/Blueprints/Core/Combat/Spells/SpellAnimations/Material/SA_Attack_Interactive/Materical/E0_ATI_Date` (`self.ATI_Date`))))))
        (:`  `
          (`KismetSystemLibrary.PrintText` (`|FormatText` "计算回合数{A} \n" _result) false false)
          (if (<= _result 0)
            (`self.Boom_Master` false)))))))

(event `Event_Torpedo_Timeline_Stop`
  ;[1 0.8136 0 1 36] 鱼雷移动
  (goto _label :!via `Stop`))

(event `self.Event_Touch_ATI`
  (params (`Show?` :type Boolean))
  ;[1 1 1] 接触到单位触发RI_UI显示
  (if `Show?`
    (if (`self.bCanShowSRUI`)
      (`self.F_Reset_Materical`)
      (`/Game/TurnBasedTactic/Blueprints/Core/Combat/Spells/SpellAnimations/Material/SA_Attack_Interactive/Torpedo/BP_TorpedoRangeIcon.Show_Toredo_Icon` (cast `/Game/TurnBasedTactic/Blueprints/Core/Combat/Spells/SpellAnimations/Material/SA_Attack_Interactive/Torpedo/BP_TorpedoRangeIcon` (`ChildActorComponent.ChildActor` (`self.Show_Range_Icon`)) :!pure true) (`.Age_Current_15_B1EF7DD84DA60BE5C40CDEBDE7AE72BA` (break `/Game/TurnBasedTactic/Blueprints/Core/Combat/Spells/SpellAnimations/Material/SA_Attack_Interactive/Materical/E_ATI_BaseState` (`.BaseState_9_997CD240407AC492B23DB296C2061696` (break `/Game/TurnBasedTactic/Blueprints/Core/Combat/Spells/SpellAnimations/Material/SA_Attack_Interactive/Materical/E0_ATI_Date` (`self.ATI_Date`))))) (`.Torpedo_Speed_12_D21B9F8C40718C08D61C7FA65F4A5EA1` (break `/Game/TurnBasedTactic/Blueprints/Core/Combat/Spells/SpellAnimations/Material/SA_Attack_Interactive/Materical/E_ATI_DateTorpedo` (`self.Torpedo_Date`)))))))

(event `self.Play_PathAnim`
  (bind _ati_date_attack_interactive_asset (break `/Game/TurnBasedTactic/Blueprints/Core/Combat/Spells/SpellAnimations/Material/SA_Attack_Interactive/Materical/E0_ATI_Date` (`self.ATI_Date`)))
  ;[1 1 1] 播放出生动画
  (bind _output_randompath (`self.F Random Path Anim` (`.Brith_Path_24_218CA4D24229C0D5DD193F81A24900F5` (break `/Game/TurnBasedTactic/Blueprints/Core/Combat/Spells/SpellAnimations/Material/SA_Attack_Interactive/Materical/E_ATI_Assets` _ati_date_attack_interactive_asset))))
  (if (`KismetSystemLibrary.IsValidClass` _output_randompath)
    (bind _returnvalue (`|SpawnActorFromClass` _output_randompath (`KismetMathLibrary.MakeTransform` (0.0 0.0 0.0)) "Undefined" "MultiplyWithRoot" null (`self.K2_GetActorLocation` (`self.Father_Unit`)) (`self.K2_GetActorLocation` self) self (0.0 0.0) null))
    (set `self.ATI_BP_Path` _returnvalue)))

(event `self.Hurt_Class`
  (params (Actor :type "Actor Object Reference"))
  ;[1 0 0] 触发鱼雷专属爆炸
  (`self.F_Boom_By_Torpedo` Actor))

(fn `F_Boom_By_Torpedo`
  (params (Actor :type "Actor Object Reference"))
  (locals (`Debug？` :type Boolean))
  (bind (_as0_bp_unit _bsuccess) (cast `/Game/TurnBasedTactic/Blueprints/Core/Units/0_BP_Unit` Actor :!pure true))
  (bind (_as0_bp_attack_interactive_ati _bsuccess_2) (cast `/Game/TurnBasedTactic/Blueprints/Core/Combat/Spells/SpellAnimations/Material/SA_Attack_Interactive/0_BP_Attack_Interactive_ATI` Actor :!pure true))
  (bind _ati_bp_path (`self.ATI_BP_Path`))
  (bind _ati_bp_path_2 (`self.ATI_BP_Path`))
  (bind _debug_ (`local.Debug？`))
  (set `local.Debug？` false)
  (if _bsuccess
    (if (!= (`/Game/TurnBasedTactic/Blueprints/Core/Units/0_BP_Unit.TeamIndex` _as0_bp_unit) (`self.TeamIndex`))
      ;[1 1 1] 鱼雷命中敌人
      (`KismetSystemLibrary.PrintText` "敌" _debug_ false)
      (`/Engine/EditorBlueprintResources/StandardMacros.IsValid` _ati_bp_path
        (:`Is Valid`
          (`self.K2_DestroyActor` _ati_bp_path))
        (:`Is Not Valid`
          _))
      (`self.Boom_Master` true _as0_bp_unit)
      (`self.Event_Torpedo_Timeline_Stop`)
      (else
        (`KismetSystemLibrary.PrintText` "友" _debug_ false)))
    (elif _bsuccess_2
      (if (!= (`self.TeamIndex`) (`/Game/TurnBasedTactic/Blueprints/Core/Combat/Spells/SpellAnimations/Material/SA_Attack_Interactive/0_BP_Attack_Interactive_ATI.TeamIndex` _as0_bp_attack_interactive_ati))
        (`KismetSystemLibrary.PrintText` "ATI_敌" (`local.Debug？`) false)
        (`self.Event_Torpedo_Timeline_Stop`)
        (`self.Boom_Master` true)
        (`self.ATI_Boom`)
        (`/Engine/EditorBlueprintResources/StandardMacros.IsValid` _ati_bp_path_2
          (:`Is Valid`
            (`self.K2_DestroyActor` _ati_bp_path_2))
          (:`Is Not Valid`
            _))
        (`/Engine/EditorBlueprintResources/StandardMacros.IsValid` _as0_bp_attack_interactive_ati
          (:`Is Valid`
            (`self.Boom_Master` _as0_bp_attack_interactive_ati true null)))
        (else
          (`KismetSystemLibrary.PrintText` "ATI_友" (`local.Debug？`) false)))
      (else
        (`KismetSystemLibrary.PrintText` "墙" (`local.Debug？`) false) ; 啥也没击中就是墙了
        (`self.Event_Torpedo_Timeline_Stop`)
        (`self.Boom_Master` true)
        (`self.ATI_Boom`)))))

(fn `Ready_Torpedo`
  (bind (_attack_interactive_asset _basestate) (break `/Game/TurnBasedTactic/Blueprints/Core/Combat/Spells/SpellAnimations/Material/SA_Attack_Interactive/Materical/E0_ATI_Date` (`self.ATI_Date`)))
  (`ChildActorComponent.SetChildActorClass` (`self.Show_Range_Icon`) "/Game/TurnBasedTactic/Blueprints/Core/Combat/Spells/SpellAnimations/Material/SA_Attack_Interactive/Torpedo/BP_TorpedoRangeIcon.BP_TorpedoRangeIcon_C")
  (`SceneComponent.SetWorldScale3D` (`self.Attack_Range`) (`KismetMathLibrary.Conv_DoubleToVector` (* (`.Blast_Radius_18_E0D57E7D444530BD4D387E9CF00DD2AA` (break `/Game/TurnBasedTactic/Blueprints/Core/Combat/Spells/SpellAnimations/Material/SA_Attack_Interactive/Materical/E_ATI_DateTorpedo` (`self.Torpedo_Date`))) 0.01)))
  ;[1 1 1] 攻击物模型
  (`StaticMeshComponent.SetStaticMesh` (`self.Mesh`) (`.Attack_Unit_SM_11_9588766540E242755F9AB49B4CB727E1` (break `/Game/TurnBasedTactic/Blueprints/Core/Combat/Spells/SpellAnimations/Material/SA_Attack_Interactive/Materical/E_ATI_Assets` _attack_interactive_asset)))
  ;[1 1 1] 碰撞体模型
  (`StaticMeshComponent.SetStaticMesh` (`self.Attack_Range`) (`.Collision_20_72BAA4F44AAAB1929629B4B325C8D08F` (break `/Game/TurnBasedTactic/Blueprints/Core/Combat/Spells/SpellAnimations/Material/SA_Attack_Interactive/Materical/E_ATI_BaseState` _basestate)))
  ;[1 1 1] 设置移动待机粒子
  (`ParticleSystemComponent.SetTemplate` (`self.P_Idle`) (`.Trail_VFX_Idle_24_8C3A840A44CB2459090463B7F2674851` (break `/Game/TurnBasedTactic/Blueprints/Core/Combat/Spells/SpellAnimations/Material/SA_Attack_Interactive/Materical/E_ATI_DateTorpedo` (`self.Torpedo_Date`))))
  ;[1 1 1] 把本鱼雷蓝图注入到TRI距离显示蓝图
  (set `/Game/TurnBasedTactic/Blueprints/Core/Combat/Spells/SpellAnimations/Material/SA_Attack_Interactive/Torpedo/BP_TorpedoRangeIcon.TRI_BP_Torpedo` self (cast `/Game/TurnBasedTactic/Blueprints/Core/Combat/Spells/SpellAnimations/Material/SA_Attack_Interactive/Torpedo/BP_TorpedoRangeIcon` (`ChildActorComponent.ChildActor` (`self.Show_Range_Icon`)) :!pure true)))

(fn `UserConstructionScript`
  (`parent.UserConstructionScript`)
  (`self.Ready_Torpedo`))