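; Spline path actor for the CrossFire open-fire attack animation, flying an AttackInteractive projectile from launch to detonation.
; It hides the projectile, waits a random delay, spawns firing VFX, then drives it along the spline with a timeline paced by spline length.
; Attack range and detonation enable once it nears the second spline point's height, shutting off its trail.
; At path end it triggers LittleBoom and cleans up; the OverTimeline logic is leftover.
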(event `self.Path_Actor_Spline_Mesh_Move`
  (bind _spline (`self.Spline`))
  (bind _spline_2 (`self.Spline`))
  (bind _attack_interactive (`self.Attack_Interactive`))
  (bind _begin_position (`self.Begin_Position`))
  (bind _spline_3 (`self.Spline`))
  (bind _attack_interactive_2 (`self.Attack_Interactive`))
  (bind _attack_interactive_3 (`self.Attack_Interactive`))
  (bind _attack_interactive_4 (`self.Attack_Interactive`))
  (bind (_returnvalue_roll _returnvalue_pitch _returnvalue_yaw) (`KismetMathLibrary.BreakRotator` (`KismetMathLibrary.FindLookAtRotation` _begin_position (`self.End_Position`))))
  (`self.K2_SetActorLocation` _attack_interactive_4 (0.0 0.0 -1e+17) false false)
  (`/Game/TurnBasedTactic/Blueprints/Core/Combat/Spells/SpellAnimations/Material/SA_Attack_Interactive/0_BP_Attack_Interactive_ATI.F_Use_Attack_Range` _attack_interactive_4 false)
  (`/Engine/EditorBlueprintResources/StandardMacros.IsValid` _attack_interactive_4
    (:`Is Valid`
      (`SceneComponent.SetVisibility` (`/Game/TurnBasedTactic/Blueprints/Core/Combat/Spells/SpellAnimations/Material/SA_Attack_Interactive/0_BP_Attack_Interactive_ATI.Mesh` _attack_interactive_4) false true) ; 先把模型隐藏
      (`KismetSystemLibrary.Delay` (`KismetMathLibrary.RandomFloatInRange` 0.0 0.5))
      (`|SpawnActorFromClass` "/Game/Effects/VFX/VFX_Blueprint/BP_VFX_ShellFireBoom.BP_VFX_ShellFireBoom_C" (`KismetMathLibrary.MakeTransform` (0.0 0.0 0.0)) "Undefined" "MultiplyWithRoot" null _begin_position (`KismetMathLibrary.MakeRotator` 0.0 _returnvalue_pitch _returnvalue_yaw) null)
      (`KismetSystemLibrary.Delay` 0.2)
      (`SceneComponent.SetVisibility` (`/Game/TurnBasedTactic/Blueprints/Core/Combat/Spells/SpellAnimations/Material/SA_Attack_Interactive/0_BP_Attack_Interactive_ATI.Mesh` (`self.Attack_Interactive`)) true true) ; 开始播放后显示模型
      (`|SpawnActorFromClass` "/Game/Effects/VFX/VFX_Blueprint/BP_VFX_TorpedoOut.BP_VFX_TorpedoOut_C" (`KismetMathLibrary.MakeTransform` (0.0 0.0 0.0)) "Undefined" "MultiplyWithRoot" null (`SplineComponent.GetLocationAtDistanceAlongSpline` _spline 0.0 "World") (`SplineComponent.GetRotationAtDistanceAlongSpline` _spline 0.1 "World") null)
      (`KismetSystemLibrary.Delay` 0.0)
      (`TimelineComponent.SetPlayRate` (`self.BaseTimeline`) (/ 1.0 (* (* (`SplineComponent.GetSplineLength` (`self.Spline`)) 0.001) (`self.Anim_Speed`)))) ; 设置动画速率
      (bind (_direction _path_rota_scales) (`Timeline|BaseTimeline` :!via `PlayFromStart`)
        (:`Update`
          (`/Engine/EditorBlueprintResources/StandardMacros.IsValid` _attack_interactive_3
            (:`Is Valid`
              (bind _returnvalue (* (`KismetMathLibrary.Fraction` (.x _path_rota_scales)) (`SplineComponent.GetSplineLength` (`self.Spline`))))
              (bind _returnvalue_2 (`SplineComponent.GetLocationAtDistanceAlongSpline` _spline_2 _returnvalue "World"))
              (bind _returnvalue_3 (`SplineComponent.GetRotationAtDistanceAlongSpline` _spline_2 _returnvalue "World"))
              (`self.K2_SetActorTransform` _attack_interactive_3 (`KismetMathLibrary.MakeTransform` _returnvalue_2 _returnvalue_3 (`KismetMathLibrary.Conv_DoubleToVector` (.z _path_rota_scales))) false false)
              (`/Engine/EditorBlueprintResources/StandardMacros.IsValid` _spline_3
                (:`Is Valid`
                  (if (not (> (* (.z (`SplineComponent.GetLocationAtSplinePoint` _spline_3 1 "World")) 0.9) (.z _returnvalue_2)))
                    (`/Engine/EditorBlueprintResources/StandardMacros.DoOnce` false
                      (:`Completed`
                        (`/Game/TurnBasedTactic/Blueprints/Core/Combat/Spells/SpellAnimations/Material/SA_Attack_Interactive/0_BP_Attack_Interactive_ATI.F_Use_Attack_Range` _attack_interactive true)
                        (`ActorComponent.Deactivate` (`/Game/TurnBasedTactic/Blueprints/Core/Combat/Spells/SpellAnimations/Material/SA_Attack_Interactive/0_BP_Attack_Interactive_ATI.P_Idle` _attack_interactive))))))))))
        (:`Finished`
          (`/Engine/EditorBlueprintResources/StandardMacros.IsValid` (`self.Attack_Interactive`)
            (:`Is Valid`
              (`self.Path_OverTime_Move` _returnvalue_3))
            (:`Is Not Valid`
              (`self.Path_Clear_Actor`)))
          (`/Engine/EditorBlueprintResources/StandardMacros.IsValid` (`self.Attack_Interactive`)
            (:`Is Valid`
              (`/Game/TurnBasedTactic/Blueprints/Core/Combat/Spells/SpellAnimations/Material/SA_Attack_Interactive/0_BP_Attack_Interactive_ATI.Little_Boom` _attack_interactive_2)
              (`/Game/TurnBasedTactic/Blueprints/Core/Combat/Spells/SpellAnimations/Material/SA_Attack_Interactive/0_BP_Attack_Interactive_ATI.Path_Anima_Over` _attack_interactive_2)
              (`self.K2_DestroyActor` _attack_interactive_2)
              (`self.Path_Clear_Actor`))))))))

(event `self.Path_OverTime_Move`
  (params (Rotator :type "Rotator Structure")))

(event `Stop_OverTimeline`
  ;[1 1 1] 没啥用了,不过先留着.
  (bind (_direction _over_ro) (`Timeline|OverTimeline` :!via `Stop`)
    (:`Update`
      (`/Engine/EditorBlueprintResources/StandardMacros.IsValid` (`self.Attack_Interactive`)
        (:`Is Valid`
          (`SceneComponent.SetRelativeScale3D` (`/Game/TurnBasedTactic/Blueprints/Core/Combat/Spells/SpellAnimations/Material/SA_Attack_Interactive/0_BP_Attack_Interactive_ATI.Attack_Range` (`self.Attack_Interactive`)) (`KismetMathLibrary.Conv_DoubleToVector` _over_ro)))))))

(fn `UserConstructionScript`
  (`parent.UserConstructionScript`))