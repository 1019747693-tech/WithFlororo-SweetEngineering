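; Rocket variant of the interactive attack object (ATI) in the turn-based tactics combat system.
; Construction sets up its blast-range collision mesh and idle trail particle from rocket data and mesh sockets.
; PlayPathAnim spawns a random path actor from the launching unit to the rocket.
; FBoomByRocket destroys that path and branches explosions for units, other ATIs (also detonated) or walls, but its event-graph call is unconnected.
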(event `self.ReceiveBeginPlay`
  (`parent.ReceiveBeginPlay`)
  (set `self.bCanBoom` true)
  (`self.F_Reset_Materical`)
  (`self.F_Use_Attack_Range` false))

(event `self.Event_Call_ATI_UnitBegin`)

(event `self.Play_PathAnim`
  (bind _ati_date_attack_interactive_asset (break `/Game/TurnBasedTactic/Blueprints/Core/Combat/Spells/SpellAnimations/Material/SA_Attack_Interactive/Materical/E0_ATI_Date` (`self.ATI_Date`)))
  ;[0 0 0] 播放起始动画.
  (bind _output_randompath (`self.F Random Path Anim` (`.Brith_Path_24_218CA4D24229C0D5DD193F81A24900F5` (break `/Game/TurnBasedTactic/Blueprints/Core/Combat/Spells/SpellAnimations/Material/SA_Attack_Interactive/Materical/E_ATI_Assets` _ati_date_attack_interactive_asset))))
  (if (`KismetSystemLibrary.IsValidClass` _output_randompath)
    (bind _returnvalue (`|SpawnActorFromClass` _output_randompath (`KismetMathLibrary.MakeTransform` (0.0 0.0 0.0)) "Undefined" "MultiplyWithRoot" null (`self.K2_GetActorLocation` (`self.Father_Unit`)) (`self.K2_GetActorLocation` self) self (0.0 0.0) null)) ; 播放path动画
    (set `self.ATI_BP_Path` _returnvalue)))

(event `self.Hurt_Class`
  (params (Actor :type "Actor Object Reference")))

(fn `F_Boom_By_Rocket`
  (params (Actor :type "Actor Object Reference"))
  (locals (`Use_Debug?` :type Boolean))
  (bind (_as0_bp_unit _bsuccess) (cast `/Game/TurnBasedTactic/Blueprints/Core/Units/0_BP_Unit` Actor :!pure true))
  (bind (_as0_bp_attack_interactive_ati _bsuccess_2) (cast `/Game/TurnBasedTactic/Blueprints/Core/Combat/Spells/SpellAnimations/Material/SA_Attack_Interactive/0_BP_Attack_Interactive_ATI` Actor :!pure true))
  (bind _use_debug_ (`local.Use_Debug?`))
  (set `local.Use_Debug?` false)
  (`self.K2_DestroyActor` (`self.ATI_BP_Path`))
  (if _bsuccess
    (`KismetSystemLibrary.PrintText` "命中unit" _use_debug_ false)
    (`self.Boom_Master` true _as0_bp_unit)
    (elif _bsuccess_2
      (`KismetSystemLibrary.PrintText` "命中ATI" _use_debug_ false)
      (`self.Boom_Master` true)
      (`self.ATI_Boom`)
      (`/Engine/EditorBlueprintResources/StandardMacros.IsValid` _as0_bp_attack_interactive_ati
        (:`Is Valid`
          (`self.Boom_Master` _as0_bp_attack_interactive_ati true null)))
      (else
        (`KismetSystemLibrary.PrintText` "墙" _use_debug_ false) ; 啥也没击中就是墙了
        (`self.Boom_Master` true)
        (`self.ATI_Boom`)))))

(fn `Ready_Rocket`
  (bind _p_idle (`self.P_Idle`))
  (bind _returnvalue_location (`KismetMathLibrary.BreakTransform` (`SceneComponent.GetSocketTransform` (`self.Mesh`) "Rocket_Head" "RTS_Actor")))
  (bind _returnvalue_location_2 (`KismetMathLibrary.BreakTransform` (`SceneComponent.GetSocketTransform` (`self.Mesh`) "Rocket_Trail" "RTS_Actor")))
  ;[1 1 1] 爆炸标识缩放
  (`SceneComponent.SetWorldScale3D` (`self.Attack_Range`) (`KismetMathLibrary.Conv_DoubleToVector` (* (`.Blast_Radius_18_E0D57E7D444530BD4D387E9CF00DD2AA` (break `/Game/TurnBasedTactic/Blueprints/Core/Combat/Spells/SpellAnimations/Material/SA_Attack_Interactive/Materical/E_ATI_DateRocket` (`self.Rocket_Date`))) 0.01)))
  ;[1 1 1] 碰撞体模型
  (`StaticMeshComponent.SetStaticMesh` (`self.Attack_Range`) (`.Collision_20_72BAA4F44AAAB1929629B4B325C8D08F` (break `/Game/TurnBasedTactic/Blueprints/Core/Combat/Spells/SpellAnimations/Material/SA_Attack_Interactive/Materical/E_ATI_BaseState` (`.BaseState_9_997CD240407AC492B23DB296C2061696` (break `/Game/TurnBasedTactic/Blueprints/Core/Combat/Spells/SpellAnimations/Material/SA_Attack_Interactive/Materical/E0_ATI_Date` (`self.ATI_Date`))))))
  ;[1 1 1] 设置移动待机粒子
  (`ParticleSystemComponent.SetTemplate` _p_idle (`.VFX_Idle_32_4356D8FA4B86A8213B1EC2A4E7EAE5FE` (break `/Game/TurnBasedTactic/Blueprints/Core/Combat/Spells/SpellAnimations/Material/SA_Attack_Interactive/Materical/E_ATI_DateRocket` (`self.Rocket_Date`))))
  (`ActorComponent.Activate` _p_idle false)
  ;[1 1 1] 设置火箭弹顶部碰撞体以及尾部拖尾粒子位置
  (`SceneComponent.K2_SetRelativeLocation` (`self.P_Idle`) _returnvalue_location_2 false false)
  (`SceneComponent.K2_SetRelativeLocation` (`self.Attack_Range`) _returnvalue_location false false))

(fn `UserConstructionScript`
  (`parent.UserConstructionScript`)
  (`self.Ready_Rocket`))