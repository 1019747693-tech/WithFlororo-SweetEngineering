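; Aircraft squadron manager for the turn-based tactics game, an attack-interactive actor that represents planes launched by a parent unit.
; BirthAircraft spawns attached planes in a jittered ring, resetting fuel and ammo by aircraft type.
; Turn events re-derive flight state from the target's team and recompute grid endpoints; movement only spawns takeoff marker actors so far.
; Helpers cover speed-limited grid steps and team-checked explosions, but path-animation and collision hookups are disconnected.
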(event `self.ReceiveBeginPlay`
  (bind _father_unit (`self.Father_Unit`))
  (`parent.ReceiveBeginPlay`)
  (`self.F_Reset_Materical`)
  (`KismetSystemLibrary.PrintText` (`|FormatText` "飞机管理器蓝图信息： \n父技能动画蓝图：{A} \n父unit：{B}" (`KismetSystemLibrary.GetDisplayName` (`self.Father_Spell_Animation`)) (`KismetSystemLibrary.GetDisplayName` _father_unit)) false true (struct :`R` 1.0 :`G` 0.401903 :`A` 1.0) 10.0)
  (`self.F_Count_Position`)
  (bind _output_rotation (`self.F_RestRotation` (`self.K2_GetActorRotation` _father_unit)))
  (`self.K2_SetActorRotation` _output_rotation)
  (`self.ATI_Move_Plane`))

(event `self.Event_Call_ATI_UnitBegin`
  ;[1 0 0] 父Unit开始行动时,刷新ACM的行动逻辑
  (bind (_eaircraftstate _target_unit) (`self.F_Get_Unit_Switch_ACM_State`))
  (set `self.Target_Unit` _target_unit)
  (set `self.EAircraftState_CurrentFlightState` _eaircraftstate))

(event `self.Event_Call_ATI_UnitOver`
  ;[1 0 0] Unit结束行动后,ATI_ACM开始行动
  (`self.F_Count_Position`)
  (`self.ATI_Move_Plane`))

(event `Change_Target`
  (params (EAircraftState_CurrentFlightState :type "/Game/TurnBasedTactic/Blueprints/Core/Combat/Spells/SpellAnimations/Material/SA_Attack_Interactive/Aircraft_Manager/Materical/EAircraftState Enum" :default "NewEnumerator5") (Target_Index :type "IntPoint Structure") (Target_Unit :type "/Game/TurnBasedTactic/Blueprints/Core/Units/0_BP_Unit Object Reference"))
  (bind (_target_index_x _target_index_y) (break `IntPoint` (`self.Target_Index`)))
  ;[0 0 0] 修改ACM的锁定目标
  (set `self.EAircraftState_CurrentFlightState` EAircraftState_CurrentFlightState)
  (set `self.Target_Index` Target_Index)
  (`/Engine/EditorBlueprintResources/StandardMacros.IsValid` Target_Unit
    (:`Is Valid`
      (set `self.Target_Unit` Target_Unit))
    (:`Is Not Valid`
      (set `self.Target_Unit` null)))
  (bind _state (`self.F_EAircraftState_State` (`self.EAircraftState_CurrentFlightState`)))
  (`KismetSystemLibrary.PrintText` (`|FormatText` "我现在的状态为{A} \n我的目标点索引为{B1}，{B2} \n我的目标为{C}" _state _target_index_x _target_index_y (`self.Target_Unit`))))

(event `ATI_Move_Plane`
  ;[1 0.8136 0 1 36] 舰载机移动
  (`KismetSystemLibrary.PrintText` (`KismetTextLibrary.Conv_ByteToText` (`self.EAircraftState_CurrentFlightState`)))
  (switch `/Game/TurnBasedTactic/Blueprints/Core/Combat/Spells/SpellAnimations/Material/SA_Attack_Interactive/Aircraft_Manager/Materical/EAircraftState` (`self.EAircraftState_CurrentFlightState`)
    (:`NewEnumerator5`
      (`|SpawnActorFromClass` "/Game/BP_TAG.BP_TAG_C" (`KismetMathLibrary.MakeTransform` (`self.K2_GetActorLocation` (`self.Father_Unit`))) "Undefined" "MultiplyWithRoot" null null)
      (`|SpawnActorFromClass` "/Game/BP_TAG.BP_TAG_C" (`KismetMathLibrary.MakeTransform` (`self.ATI_End_position`)) "Undefined" "MultiplyWithRoot" null null))))

(event `self.Event_Touch_ATI`
  (params (`Show?` :type Boolean))
  ;[1 1 1] 接触到单位触发RI_UI显示
  (if `Show?`
    (if (`self.bCanShowSRUI`)
      (`self.F_Reset_Materical`)
      (`/Game/TurnBasedTactic/Blueprints/Core/Combat/Spells/SpellAnimations/Material/SA_Attack_Interactive/Torpedo/BP_TorpedoRangeIcon.Show_Toredo_Icon` (cast `/Game/TurnBasedTactic/Blueprints/Core/Combat/Spells/SpellAnimations/Material/SA_Attack_Interactive/Torpedo/BP_TorpedoRangeIcon` (`ChildActorComponent.ChildActor` (`self.Show_Range_Icon`)) :!pure true) (`.Age_Current_15_B1EF7DD84DA60BE5C40CDEBDE7AE72BA` (break `/Game/TurnBasedTactic/Blueprints/Core/Combat/Spells/SpellAnimations/Material/SA_Attack_Interactive/Materical/E_ATI_BaseState` (`.BaseState_9_997CD240407AC492B23DB296C2061696` (break `/Game/TurnBasedTactic/Blueprints/Core/Combat/Spells/SpellAnimations/Material/SA_Attack_Interactive/Materical/E0_ATI_Date` (`self.ATI_Date`))))) (`.Torpedo_Speed_12_D21B9F8C40718C08D61C7FA65F4A5EA1` (break `/Game/TurnBasedTactic/Blueprints/Core/Combat/Spells/SpellAnimations/Material/SA_Attack_Interactive/Materical/E_ATI_DateTorpedo` (`self.Torpedo_Date`)))))))

(event `self.Play_PathAnim`
  ;[1 1 1] 播放出生动画
)

(event `self.Hurt_Class`
  (params (Actor :type "Actor Object Reference"))
  ;[1 0 0] 触发鱼雷专属爆炸
)

(fn `Birth Aircraft`
  (locals (Rebulid_Postion :type "Array of Vector Structure"))
  (bind _squadronsize (`self.SquadronSize`))
  (bind _returnvalue (`KismetMathLibrary.Lerp` 0.0 55.0 (/ _squadronsize 3)))
  (bind _returnvalue_2 (+ (`KismetMathLibrary.RandomFloatInRange` (* _returnvalue -0.1) (* _returnvalue 0.1)) _returnvalue))
  (`self.F_Ready_ACM` true)
  (set `self.EAircraftState_CurrentFlightState` "NewEnumerator5")
  (`KismetArrayLibrary.Array_Clear` (`self.Child_AirCraft`))
  (`KismetArrayLibrary.Array_Clear` (`local.Rebulid_Postion`))
  (for _index (range _squadronsize)
    (bind _returnvalue_3 (* (* (/ 360 _squadronsize) _index) (/ (`KismetMathLibrary.GetPI`) 180.0)))
    (`KismetArrayLibrary.Array_Add` (`local.Rebulid_Postion`) (`KismetMathLibrary.MakeVector` (* _returnvalue_2 (`KismetMathLibrary.Cos` _returnvalue_3)) (* (`KismetMathLibrary.Sin` _returnvalue_3) _returnvalue_2) (`KismetMathLibrary.RandomFloatInRange` -50.0 50.0))))
  (for _array_element (`local.Rebulid_Postion`)
    ;[1 1 1] 生成小飞机
    (bind _returnvalue_4 (`|SpawnActorFromClass` (`self.AirCraft_Type`) (`KismetMathLibrary.MakeTransform` _array_element (struct :`Yaw` 90.0) (`KismetMathLibrary.Conv_DoubleToVector` (`KismetMathLibrary.FMax` (- 1.0 (* 0.2 _squadronsize)) 0.4))) "Undefined" "MultiplyWithRoot" null self 30.0 0.0 (`self.TeamIndex`) (`self.Father_Unit`) (`self.Father_Spell_Animation`) null))
    (`self.K2_AttachToActor` _returnvalue_4 self "None" "KeepRelative" "KeepRelative" "KeepRelative" true)))

(fn `F_Boom_By_ACM`
  (params (Actor :type "Actor Object Reference"))
  (locals (`Debug？` :type Boolean))
  (bind (_as0_bp_unit _bsuccess) (cast `/Game/TurnBasedTactic/Blueprints/Core/Units/0_BP_Unit` Actor :!pure true))
  (bind (_as0_bp_attack_interactive_ati _bsuccess_2) (cast `/Game/TurnBasedTactic/Blueprints/Core/Combat/Spells/SpellAnimations/Material/SA_Attack_Interactive/0_BP_Attack_Interactive_ATI` Actor :!pure true))
  (bind _ati_bp_path (`self.ATI_BP_Path`))
  (bind _ati_bp_path_2 (`self.ATI_BP_Path`))
  (set `local.Debug？` true)
  (if _bsuccess
    (if (!= (`/Game/TurnBasedTactic/Blueprints/Core/Units/0_BP_Unit.TeamIndex` _as0_bp_unit) (`self.TeamIndex`))
      (`KismetSystemLibrary.PrintText` "敌" true false)
      (`/Engine/EditorBlueprintResources/StandardMacros.IsValid` _ati_bp_path
        (:`Is Valid`
          (`self.K2_DestroyActor` _ati_bp_path))
        (:`Is Not Valid`
          _))
      (`self.Boom_Master` true _as0_bp_unit)
      (else
        (`KismetSystemLibrary.PrintText` "友" (`local.Debug？`) false)))
    (elif _bsuccess_2
      (if (!= (`self.TeamIndex`) (`/Game/TurnBasedTactic/Blueprints/Core/Combat/Spells/SpellAnimations/Material/SA_Attack_Interactive/0_BP_Attack_Interactive_ATI.TeamIndex` _as0_bp_attack_interactive_ati))
        (`KismetSystemLibrary.PrintText` "ATI_敌" (`local.Debug？`) false)
        (`self.Boom_Master` true)
        (`self.ATI_Boom`)
        (`/Engine/EditorBlueprintResources/StandardMacros.IsValid` _ati_bp_path_2
          (:`Is Valid`
            (`self.K2_DestroyActor` _ati_bp_path_2))
          (:`Is Not Valid`
            _))
        (`/Engine/EditorBlueprintResources/StandardMacros.IsValid` _as0_bp_attack_interactive_ati
          (:`Is Valid`
            (`self.Boom_Master` _as0_bp_attack_interactive_ati true null)))
        (else
          (`KismetSystemLibrary.PrintText` "ATI_友" (`local.Debug？`) false)))
      (else
        (`KismetSystemLibrary.PrintText` "墙" (`local.Debug？`) false) ; 啥也没击中就是墙了
        (`self.Boom_Master` true)
        (`self.ATI_Boom`)))))

(fn `F_Count_Position`
  (switch `/Game/TurnBasedTactic/Blueprints/Core/Combat/Spells/SpellAnimations/Material/SA_Attack_Interactive/Aircraft_Manager/Materical/EAircraftState` (`self.EAircraftState_CurrentFlightState`)
    (:`NewEnumerator5`
      (set `self.ATI_Begin_position` (+ (`self.K2_GetActorLocation` (`self.Father_Unit`)) (0.0 0.0 100.0)))
      (bind _returnvalue (`GameplayStatics.GetActorOfClass` "/Game/TurnBasedTactic/Blueprints/Core/Grid/BP_Grid.BP_Grid_C"))
      (set `self.ATI_End_position` (`/Game/TurnBasedTactic/Blueprints/Core/Grid/BP_Grid.GetTileLocationFromGridIndex` _returnvalue (`self.Target_Index`))))
    (:`NewEnumerator6`
      (set `self.ATI_Begin_position` (`self.K2_GetActorLocation` self) :!label _label)
      (bind _returnvalue_2 (`GameplayStatics.GetActorOfClass` "/Game/TurnBasedTactic/Blueprints/Core/Grid/BP_Grid.BP_Grid_C"))
      (set `self.ATI_End_position` (`/Game/TurnBasedTactic/Blueprints/Core/Grid/BP_Grid.GetTileLocationFromGridIndex` _returnvalue_2 (`self.Target_Index`))))
    (:`NewEnumerator1`
      (goto _label))
    (:`NewEnumerator2`
      (goto _label))))

(fn `F_EAircraftState_State`
  (params (EAircraftState_CurrentFlightState :type "/Game/TurnBasedTactic/Blueprints/Core/Combat/Spells/SpellAnimations/Material/SA_Attack_Interactive/Aircraft_Manager/Materical/EAircraftState Enum" :default "NewEnumerator5"))
  (returns (State :type Text))
  (locals (Out_State :type Text))
  (switch `/Game/TurnBasedTactic/Blueprints/Core/Combat/Spells/SpellAnimations/Material/SA_Attack_Interactive/Aircraft_Manager/Materical/EAircraftState` EAircraftState_CurrentFlightState
    (:`NewEnumerator5`
      (set `local.Out_State` "起飞"))
    (:`NewEnumerator6`
      (set `local.Out_State` "空中警戒"))
    (:`NewEnumerator1`
      (set `local.Out_State` "护卫"))
    (:`NewEnumerator2`
      (set `local.Out_State` "袭击"))
    (:`NewEnumerator0`
      (set `local.Out_State` "返航")))
  (return (`local.Out_State`)))

(fn `F_Get_ACSpeed_Target_Position`
  (params (Begin_Position :type "Vector Structure") (Over_Position :type "Vector Structure"))
  (returns (Target_Position :type "Vector Structure"))
  (bind _returnvalue (+ (* (`KismetMathLibrary.Normal` (- Begin_Position Over_Position)) (`self.FlightSpeed`)) Over_Position))
  (switch `/Game/TurnBasedTactic/Blueprints/Core/Combat/Spells/SpellAnimations/Material/SA_Attack_Interactive/Aircraft_Manager/Materical/EAircraftState` (`self.EAircraftState_CurrentFlightState`)
    (:`NewEnumerator5`
      ;[1 1 1] 起飞的时候距离减半
      (bind _output_index_position (`self.F_Position_To_IndexPosition` (/ _returnvalue 2.0)))
      (return _output_index_position))
    (:`NewEnumerator6`
      _)
    (:`NewEnumerator1`
      _)
    (:`NewEnumerator2`
      _)
    (:`NewEnumerator0`
      _))
  (if (> (+ (`KismetMathLibrary.Abs` (.x (- Begin_Position Over_Position))) (`KismetMathLibrary.Abs` (.y (- Begin_Position Over_Position))) (`KismetMathLibrary.Abs` (.z (- Begin_Position Over_Position)))) (+ (`KismetMathLibrary.Abs` (.x (- _returnvalue Over_Position))) (`KismetMathLibrary.Abs` (.y (- _returnvalue Over_Position))) (`KismetMathLibrary.Abs` (.z (- _returnvalue Over_Position)))))
    ;[1 1 1] 注释
    (bind _output_index_position_2 (`self.F_Position_To_IndexPosition` _returnvalue))
    (return _output_index_position_2)
    (else
      (bind _output_index_position_3 (`self.F_Position_To_IndexPosition` Over_Position))
      (return _output_index_position_3))))

(fn `F_Get_Unit_Switch_ACM_State`
  (returns (EAircraftState :type "/Game/TurnBasedTactic/Blueprints/Core/Combat/Spells/SpellAnimations/Material/SA_Attack_Interactive/Aircraft_Manager/Materical/EAircraftState Enum") (Target_Unit :type "/Game/TurnBasedTactic/Blueprints/Core/Units/0_BP_Unit Object Reference"))
  (bind _target_unit (`self.Target_Unit`))
  (`/Engine/EditorBlueprintResources/StandardMacros.IsValid` _target_unit
    (:`Is Valid`
      (if (== (`/Game/TurnBasedTactic/Blueprints/Core/Units/0_BP_Unit.TeamIndex` (`self.Father_Unit`)) (`/Game/TurnBasedTactic/Blueprints/Core/Units/0_BP_Unit.TeamIndex` _target_unit))
        (`KismetSystemLibrary.PrintText` "护卫")
        (if (== (`self.Target_Unit`) (`self.Father_Unit`))
          (return "NewEnumerator0" (`self.Target_Unit`))
          (else
            (return "NewEnumerator1" (`self.Target_Unit`))))
        (else
          (`KismetSystemLibrary.PrintText` "袭击")
          (return "NewEnumerator2" (`self.Target_Unit`)))))
    (:`Is Not Valid`
      (`KismetSystemLibrary.PrintText` "空中警戒")
      (return "NewEnumerator6" null))))

(fn `F_Ready_ACM`
  (params (`Remake_Ammo？` :type Boolean :default true))
  ;[1 1 1] 重置燃料
  (set `self.CurrentFuel` (`self.MaxFuel`))
  (set `self.bIsOutOfFuel` false) ; 重置燃油状态
  (if `Remake_Ammo？`
    ;[1 1 1] 其中轰炸机，空中炮艇，UFO，加油机，会获得子弹，但是其余舰载机不会(因为也用不到)，但是注意不能让加油机给加油机补充
    (switch `/Game/TurnBasedTactic/Blueprints/Core/Combat/Spells/SpellAnimations/Material/SA_Attack_Interactive/Aircraft_Manager/Materical/EAircraftType` (defaults `Object` (`self.AirCraft_Type`))
      (:`NewEnumerator5`
        (set `self.CurrentAmmo` 0 :!label _label))
      (:`NewEnumerator6`
        (set `self.CurrentAmmo` (`self.MaxAmmo`) :!label _label_2))
      (:`NewEnumerator7`
        (goto _label))
      (:`NewEnumerator8`
        (goto _label))
      (:`NewEnumerator9`
        (goto _label_2))
      (:`NewEnumerator10`
        (goto _label))
      (:`NewEnumerator13`
        (goto _label_2))
      (:`NewEnumerator11`
        (goto _label_2)))))

(fn `OnRep_SquadronSize`)

(fn `UserConstructionScript`
  (`parent.UserConstructionScript`))