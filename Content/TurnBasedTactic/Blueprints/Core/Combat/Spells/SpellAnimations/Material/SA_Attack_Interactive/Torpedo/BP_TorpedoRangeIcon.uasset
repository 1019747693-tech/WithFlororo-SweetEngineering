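; Range indicator actor that previews a torpedo's estimated path as a row of plane icons tinted with the torpedo's index color.
; Show_Toredo_Icon derives path length from age and speed, placing evenly spaced points forward until a line trace hits.
; It spawns a mesh component per point, then a timeline animates Y scale and the torpedo's range material opacity.
; A flag blocks retriggering until the timeline finishes.
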(event `self.ReceiveBeginPlay`
  (bind _returnvalue (`KismetMaterialLibrary.CreateDynamicMaterialInstance` "/Game/TurnBasedTactic/Blueprints/Core/Combat/Spells/SpellAnimations/Material/SA_Attack_Interactive/Torpedo/BaseMatercail/M_RangePlane_Inst.M_RangePlane_Inst"))
  (`MaterialInstanceDynamic.SetVectorParameterValue` _returnvalue "Index_Color" (`/Game/TurnBasedTactic/Blueprints/Core/Combat/Spells/SpellAnimations/Material/SA_Attack_Interactive/0_BP_Attack_Interactive_ATI.IndexColor` (`self.TRI_BP_Torpedo`)))
  (set `self.Index_Mat` _returnvalue))

(event `Show_Toredo_Icon`
  (params (Age_Current :type Integer) (Torpedo_Speed :type Integer))
  (bind _returnvalue (+ (`self.K2_GetActorLocation`) (0.0 0.0 100.0)))
  ;[1 1 1] 鱼雷预估路径icon生成
  (if (`self.RI_CanJumpUI?`)
    (`KismetArrayLibrary.Array_Clear` (`self.Rebulid_Postion`))
    (set `self.RI_CanJumpUI?` false)
    (for _index (range (+ (* (- Age_Current 1) Torpedo_Speed) 1)) :!label _label
      (bind _returnvalue_2 (* _index 200))
      (`KismetArrayLibrary.Array_Add` (`self.Rebulid_Postion`) (`KismetMathLibrary.MakeVector` _returnvalue_2 0.0 2.0))
      (bind (_outhit _returnvalue_3) (`KismetSystemLibrary.LineTraceSingle` _returnvalue (+ _returnvalue (+ (* (`SceneComponent.GetForwardVector` (`self.DefaultSceneRoot`)) _returnvalue_2) (0.0 0.0 20.0))) "TraceTypeQuery3"))
      (if _returnvalue_3
        (`self.Break_Loop`)))
    ;;[1 1 1] 生成模型组
    (for _array_element (`self.Rebulid_Postion`)
      (bind _returnvalue_4 (`AddComponent|NODE_AddStaticMeshComponent-3` :`RelativeTransform` (`KismetMathLibrary.MakeTransform` _array_element)))
      (`PrimitiveComponent.SetMaterial` _returnvalue_4 0 (`self.Index_Mat`)))
    (bind (_direction _size) (`Timeline|时间轴` :!via `PlayFromStart`)
      (:`Update`
        (`self.SetActorScale3D` self (`KismetMathLibrary.MakeVector` 1.0 _size 1.0))
        (`MaterialInstanceDynamic.SetScalarParameterValue` (`/Game/TurnBasedTactic/Blueprints/Core/Combat/Spells/SpellAnimations/Material/SA_Attack_Interactive/0_BP_Attack_Interactive_ATI.Attack Range Mat` (`self.TRI_BP_Torpedo`)) "Opi_Master" _size))
      (:`Finished`
        (set `self.RI_CanJumpUI?` true)))))

(event `Break_Loop`
  ;[1 1 1] 鱼雷预估路径icon生成
  (goto _label :!via `Break`))

(fn `UserConstructionScript`)