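; Range indicator actor for the naval mine in the turn-based combat, pairing a ground plane with a WB_Naval_Mine widget.
; Jump_UI tints the plane's dynamic material, shows both components, passes the mine's current age to the widget and plays its jump animation.
; A timeline scales the plane, then hides both on finish, with a flag blocking retriggers while it plays.
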(event `self.ReceiveBeginPlay`
  (bind _plane (`self.Plane`))
  (bind _returnvalue (`PrimitiveComponent.CreateDynamicMaterialInstance` _plane 0 (`PrimitiveComponent.GetMaterial` _plane 0) "None"))
  (set `self.Plane_Mat` _returnvalue))

(event `Jump_UI`
  (params (`Is_Player_NavalMine?` :type Boolean) (UI_Age_Current :type Integer) (Index_Color :type "LinearColor Structure"))
  (bind _aswb_naval_mine (cast `/Game/TurnBasedTactic/Blueprints/Core/Combat/Spells/SpellAnimations/Material/SA_Attack_Interactive/Naval_Mine/BaseMatercail/WB_Naval_Mine` (`WidgetComponent.GetWidget` (`self.WB_Naval_Mine`)) :!pure true))
  (if (`self.CanJumpUI?`)
    (`MaterialInstanceDynamic.SetVectorParameterValue` (`self.Plane_Mat`) "Index_Color" Index_Color)
    (`SceneComponent.SetVisibility` (`self.WB_Naval_Mine`) true false)
    (`SceneComponent.SetVisibility` (`self.Plane`) true false)
    (set `self.CanJumpUI?` false)
    (set `/Game/TurnBasedTactic/Blueprints/Core/Combat/Spells/SpellAnimations/Material/SA_Attack_Interactive/Naval_Mine/BaseMatercail/WB_Naval_Mine.UI_Age_Current` UI_Age_Current _aswb_naval_mine)
    (`/Game/TurnBasedTactic/Blueprints/Core/Combat/Spells/SpellAnimations/Material/SA_Attack_Interactive/Naval_Mine/BaseMatercail/WB_Naval_Mine.Jump_UI_Anim` _aswb_naval_mine)
    (bind (_direction _size) (`Timeline|时间轴` :!via `PlayFromStart`)
      (:`Update`
        (`SceneComponent.SetWorldScale3D` (`self.Plane`) (`KismetMathLibrary.Conv_DoubleToVector` _size)))
      (:`Finished`
        (set `self.CanJumpUI?` true)
        (`self.Show_UI_Visibility` false)))))

(event `Show_UI_Visibility`
  (params (UI_Plane_Visibility :type Boolean))
  (`SceneComponent.SetVisibility` (`self.WB_Naval_Mine`) UI_Plane_Visibility false)
  (`SceneComponent.SetVisibility` (`self.Plane`) UI_Plane_Visibility false))

(fn `UserConstructionScript`)