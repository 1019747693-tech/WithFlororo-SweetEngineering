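; Aircraft path actor that moves an AttackInteractive actor along a procedurally generated spline in a turn-based tactics game.
; The construction script builds a curved turn toward EndPosition using dot products, then rebuilds it from an adjusted endpoint.
; BaseTimeline drives the transform at a rate scaled by spline length and AnimSpeed.
; OverTimeline handles aligning to FatherUnit and re-enabling attack range, but its PlayFromStart call is unreachable.
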(event `self.Path_Actor_Spline_Mesh_Move`
  (bind _spline (`self.Spline`))
  (bind _attack_interactive (`self.Attack_Interactive`))
  (`TimelineComponent.SetPlayRate` (`self.BaseTimeline`) (/ 1.0 (* (* (`SplineComponent.GetSplineLength` (`self.Spline`)) 0.001) (`self.Anim_Speed`)))) ; 设置动画速率
  (bind (_direction _path_rota_scales) (`Timeline|BaseTimeline` :!via `PlayFromStart` :!label _label)
    (:`Update`
      (`/Engine/EditorBlueprintResources/StandardMacros.IsValid` _attack_interactive
        (:`Is Valid`
          (bind _returnvalue (* (`KismetMathLibrary.Fraction` (.x _path_rota_scales)) (`SplineComponent.GetSplineLength` (`self.Spline`))))
          (bind _returnvalue_2 (`SplineComponent.GetRotationAtDistanceAlongSpline` _spline _returnvalue "World"))
          (`self.K2_SetActorTransform` _attack_interactive (`KismetMathLibrary.MakeTransform` (`SplineComponent.GetLocationAtDistanceAlongSpline` _spline _returnvalue "World") _returnvalue_2 (`KismetMathLibrary.Conv_DoubleToVector` (.z _path_rota_scales))) false false))))
    (:`Finished`
      (`/Engine/EditorBlueprintResources/StandardMacros.IsValid` (`self.Attack_Interactive`)
        (:`Is Valid`
          (`self.Path_OverTime_Move` _returnvalue_2))
        (:`Is Not Valid`
          (`self.Path_Clear_Actor`))))))

(event `Stop_BaseTimeLine`
  (goto _label :!via `Stop`))

(event `self.Path_OverTime_Move`
  (params (Rotator :type "Rotator Structure")))

(event `Stop_OverTimeline`
  (bind _attack_interactive (`self.Attack_Interactive`))
  (bind (_direction _over_ro) (`Timeline|OverTimeline` :!via `Stop`)
    (:`Update`
      (`/Engine/EditorBlueprintResources/StandardMacros.IsValid` (`self.Attack_Interactive`)
        (:`Is Valid`
          (`self.K2_SetActorTransform` (`self.Attack_Interactive`) (`KismetMathLibrary.MakeTransform` (`SplineComponent.GetLocationAtDistanceAlongSpline` (`self.Spline`) (`SplineComponent.GetSplineLength` (`self.Spline`)) "World") (`KismetMathLibrary.RLerp` (stale `self.Path_OverTime_Move` Rotator) (`self.K2_GetActorRotation` (`/Game/TurnBasedTactic/Blueprints/Core/Combat/Spells/SpellAnimations/Material/SA_Attack_Interactive/0_BP_Attack_Interactive_ATI.Father_Unit` (`self.Attack_Interactive`))) _over_ro true)) false false))))
    (:`Finished`
      (`/Engine/EditorBlueprintResources/StandardMacros.IsValid` (`self.Attack_Interactive`)
        (:`Is Valid`
          (`/Game/TurnBasedTactic/Blueprints/Core/Combat/Spells/SpellAnimations/Material/SA_Attack_Interactive/0_BP_Attack_Interactive_ATI.F_Use_Attack_Range` _attack_interactive true)
          (`/Game/TurnBasedTactic/Blueprints/Core/Combat/Spells/SpellAnimations/Material/SA_Attack_Interactive/0_BP_Attack_Interactive_ATI.Path_Anima_Over` _attack_interactive)
          (`self.Path_Clear_Actor`))))))

(event `self.Path_Stop_Timeline`
  ;[1 1 1] 停止时间轴动画
  (`self.Stop_BaseTimeLine`)
  (`self.Stop_OverTimeline`)
  (`self.Path_Clear_Actor`))

(fn `F_First_Set_Spline`
  (params (Input_End_Postion :type "Vector Structure"))
  (returns (First_Spline :type "SplineComponent Object Reference") (OutPut_End_Postion :type "Vector Structure"))
  (bind _spline (`self.Spline`))
  (bind _returnvalue (`KismetMathLibrary.Normal` (- (`local.Input_End_Postion`) (`self.Begin_Position`))))
  (bind _returnvalue_2 (< (`KismetMathLibrary.Vector_Distance` (`local.Input_End_Postion`) (`self.Begin_Position`)) (`KismetMathLibrary.Vector_Distance` (`self.Begin_Position`) (`|GetArrayItem` (`self.Position`)))))
  ;[1 1 1] 清理掉所有点
  (`SplineComponent.ClearSplinePoints` (`self.Spline`) true)
  (`KismetArrayLibrary.Array_Clear` (`self.Position`))
  (set `self.Front_Or_Back` (`KismetMathLibrary.Dot_VectorVector` _returnvalue (`SceneComponent.GetForwardVector` (`self.DefaultSceneRoot`)))) ; 确定前后,1为最前最后
  (set `self.Left_Or_Right` (`KismetMathLibrary.Dot_VectorVector` _returnvalue (`SceneComponent.GetRightVector` (`self.DefaultSceneRoot`)))) ; 确定左右,1为最左最右
  (set `self.FB_Lerp` (- 1.0 (/ (+ (`self.Front_Or_Back`) 1.0) 2.0)))
  (for _index (range 1 5)
    (`KismetArrayLibrary.Array_Add` (`self.Position`) (+ (* (/ (`KismetMathLibrary.Conv_IntToDouble` _index) 6.0) (* (`KismetMathLibrary.GreaterGreater_VectorRotator` (`SceneComponent.GetForwardVector` (`self.DefaultSceneRoot`)) (`KismetMathLibrary.MakeRotator` 0.0 0.0 (* (* _index (/ (`KismetMathLibrary.RadiansToDegrees` (`KismetMathLibrary.Acos` (`KismetMathLibrary.Dot_VectorVector` (`KismetMathLibrary.Normal` (- (`local.Input_End_Postion`) (`self.Begin_Position`))) (`SceneComponent.GetForwardVector` (`self.DefaultSceneRoot`))))) 6.0)) (`KismetMathLibrary.SignOfFloat` (`self.Left_Or_Right`))))) (`self.TurnRate `))) (`self.Begin_Position`))))
  (`KismetArrayLibrary.Array_Reverse` (`self.Position`))
  (if (not _returnvalue_2)
    (`SplineComponent.AddSplinePointAtIndex` (`self.Spline`) (`local.Input_End_Postion`) 0 "Local" true))
  (for _array_element (`self.Position`)
    (`SplineComponent.AddSplinePointAtIndex` (`self.Spline`) _array_element 0 "Local" true))
  (`SplineComponent.AddSplinePointAtIndex` _spline (`self.Begin_Position`) 0 "Local" true)
  (if (not _returnvalue_2)
    (`SplineComponent.AddSplinePointAtIndex` _spline (* (+ (`SplineComponent.GetLocationAtSplinePoint` _spline 4 "Local") (`local.Input_End_Postion`)) 0.5) 5 "Local" true))
  (return (`self.Spline`) (`local.Input_End_Postion`)))

(fn `UserConstructionScript`
  (`parent.UserConstructionScript`)
  (bind _first_spline (`self.F_First_Set_Spline` (`self.End_Position`)))
  (bind _index_position (`self.F_SetPosit_To_IndexPosit` (`SplineComponent.GetLocationAtDistanceAlongSpline` _first_spline (`self.Distance`) "Local")))
  (`self.F_First_Set_Spline` _index_position))