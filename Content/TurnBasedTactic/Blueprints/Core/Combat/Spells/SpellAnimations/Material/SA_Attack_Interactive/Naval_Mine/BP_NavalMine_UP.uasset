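; BP_NavalMine_UP is a spell-animation path actor that plays the rise-up motion of an interactive naval mine attack object.
; On move, it hides the AttackInteractive mesh, then reveals it with its outline after a short random delay.
; A half-speed NavalMine timeline lifts the object from below to its original location while driving its uniform scale.
; Finishing notifies AttackInteractive and clears the path actor, while a stop event clears it and halts the timeline.
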(event `self.Path_Actor_Spline_Mesh_Move`
  (bind _actor_postion (`self.Actor_Postion`))
  (bind _attack_interactive (`self.Attack_Interactive`))
  (bind (_returnvalue_location _returnvalue_rotation) (`KismetMathLibrary.BreakTransform` (`self.GetTransform` _attack_interactive)))
  (`SceneComponent.SetVisibility` (`/Game/TurnBasedTactic/Blueprints/Core/Combat/Spells/SpellAnimations/Material/SA_Attack_Interactive/0_BP_Attack_Interactive_ATI.Mesh` (`self.Attack_Interactive`)) false true)
  (`KismetSystemLibrary.Delay` (`KismetMathLibrary.RandomFloatInRange` 0.1 0.2))
  (`SceneComponent.SetVisibility` (`/Game/TurnBasedTactic/Blueprints/Core/Combat/Spells/SpellAnimations/Material/SA_Attack_Interactive/0_BP_Attack_Interactive_ATI.Mesh` (`self.Attack_Interactive`)) true false)
  (`SceneComponent.SetVisibility` (`/Game/TurnBasedTactic/Blueprints/Core/Combat/Spells/SpellAnimations/Material/SA_Attack_Interactive/0_BP_Attack_Interactive_ATI.OutLineMesh` (`self.Attack_Interactive`)) true false)
  (set `self.Actor_Postion` (`self.K2_GetActorLocation` (`self.Attack_Interactive`)))
  (`TimelineComponent.SetPlayRate` (`self.NavalMine`) 0.5)
  (bind (_direction _x_z_y_size_z__) (`Timeline|NavalMine` :!via `PlayFromStart` :!label _label)
    (:`Update`
      (`self.K2_SetActorTransform` (`self.Attack_Interactive`) (`KismetMathLibrary.MakeTransform` (`KismetMathLibrary.VLerp` (- _actor_postion (0.0 0.0 100.0)) _actor_postion (.x _x_z_y_size_z__)) _returnvalue_rotation (`KismetMathLibrary.Conv_DoubleToVector` (.y _x_z_y_size_z__))) false false))
    (:`Finished`
      (`/Engine/EditorBlueprintResources/StandardMacros.IsValid` _attack_interactive
        (:`Is Valid`
          _)
        (:`Is Not Valid`
          _))
      (`/Game/TurnBasedTactic/Blueprints/Core/Combat/Spells/SpellAnimations/Material/SA_Attack_Interactive/0_BP_Attack_Interactive_ATI.Path_Anima_Over` _attack_interactive)
      (`self.Path_Clear_Actor`))))

(event `self.Path_Stop_Timeline`
  (`self.Path_Clear_Actor`)
  (goto _label :!via `Stop`))

(fn `UserConstructionScript`
  (`parent.UserConstructionScript`))