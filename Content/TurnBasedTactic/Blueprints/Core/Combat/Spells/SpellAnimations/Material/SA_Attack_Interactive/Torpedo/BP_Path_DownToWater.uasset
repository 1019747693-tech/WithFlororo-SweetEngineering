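; Spline path actor for a torpedo attack animation in turn-based combat, moving an AttackInteractive from launch down to the water.
; After a random stagger with the mesh hidden, it spawns launch VFX and reveals the mesh.
; A timeline scaled by spline length and AnimSpeed drives position, rotation and scale along the spline.
; At the end it calls Splash, blends rotation to the owning unit's, signals path completion and clears itself.
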(event `self.Path_Actor_Spline_Mesh_Move`
  (bind _spline (`self.Spline`))
  (bind _spline_2 (`self.Spline`))
  (bind _attack_interactive (`self.Attack_Interactive`))
  (bind _attack_interactive_2 (`self.Attack_Interactive`))
  (`self.K2_SetActorLocation` _attack_interactive_2 (0.0 0.0 -1e+17) false false)
  (`/Game/TurnBasedTactic/Blueprints/Core/Combat/Spells/SpellAnimations/Material/SA_Attack_Interactive/0_BP_Attack_Interactive_ATI.F_Use_Attack_Range` _attack_interactive_2 false)
  (`/Engine/EditorBlueprintResources/StandardMacros.IsValid` _attack_interactive_2
    (:`Is Valid`
      (`SceneComponent.SetVisibility` (`/Game/TurnBasedTactic/Blueprints/Core/Combat/Spells/SpellAnimations/Material/SA_Attack_Interactive/0_BP_Attack_Interactive_ATI.Mesh` _attack_interactive_2) false true) ; 先把模型隐藏
      (`KismetSystemLibrary.Delay` (`KismetMathLibrary.RandomFloatInRange` 0.0 0.5))
      (`SceneComponent.SetVisibility` (`/Game/TurnBasedTactic/Blueprints/Core/Combat/Spells/SpellAnimations/Material/SA_Attack_Interactive/0_BP_Attack_Interactive_ATI.Mesh` (`self.Attack_Interactive`)) true true) ; 开始播放后显示模型
      (`|SpawnActorFromClass` "/Game/Effects/VFX/VFX_Blueprint/BP_VFX_TorpedoOut.BP_VFX_TorpedoOut_C" (`KismetMathLibrary.MakeTransform` (0.0 0.0 0.0)) "Undefined" "MultiplyWithRoot" null (`SplineComponent.GetLocationAtDistanceAlongSpline` _spline 0.0 "World") (`SplineComponent.GetRotationAtDistanceAlongSpline` _spline 0.1 "World") null)
      (`KismetSystemLibrary.Delay` 0.15)
      (`/Game/TurnBasedTactic/Blueprints/Core/Combat/Spells/SpellAnimations/Material/SA_Attack_Interactive/0_BP_Attack_Interactive_ATI.F_Use_Attack_Range` (`self.Attack_Interactive`) true)
      (`TimelineComponent.SetPlayRate` (`self.BaseTimeline`) (/ 1.0 (* (* (`SplineComponent.GetSplineLength` (`self.Spline`)) 0.001) (`self.Anim_Speed`)))) ; 设置动画速率
      (bind (_direction _path_rota_scales) (`Timeline|BaseTimeline` :!via `PlayFromStart` :!label _label)
        (:`Update`
          (`/Engine/EditorBlueprintResources/StandardMacros.IsValid` _attack_interactive
            (:`Is Valid`
              (bind _returnvalue (* (`KismetMathLibrary.Fraction` (.x _path_rota_scales)) (`SplineComponent.GetSplineLength` (`self.Spline`))))
              (bind _returnvalue_2 (`SplineComponent.GetRotationAtDistanceAlongSpline` _spline_2 _returnvalue "World"))
              (`self.K2_SetActorTransform` _attack_interactive (`KismetMathLibrary.MakeTransform` (`SplineComponent.GetLocationAtDistanceAlongSpline` _spline_2 _returnvalue "World") _returnvalue_2 (`KismetMathLibrary.Conv_DoubleToVector` (.z _path_rota_scales))) false false))))
        (:`Finished`
          (`/Engine/EditorBlueprintResources/StandardMacros.IsValid` (`self.Attack_Interactive`)
            (:`Is Valid`
              (`self.Path_OverTime_Move` _returnvalue_2))
            (:`Is Not Valid`
              (`self.Path_Clear_Actor`))))))))

(event `Stop_BaseTimeLine`
  (goto _label :!via `Stop`))

(event `self.Path_OverTime_Move`
  (params (Rotator :type "Rotator Structure"))
  (bind _attack_interactive (`self.Attack_Interactive`))
  (bind _attack_interactive_2 (`self.Attack_Interactive`))
  (`/Engine/EditorBlueprintResources/StandardMacros.IsValid` (`self.Attack_Interactive`)
    (:`Is Valid`
      (`/Game/TurnBasedTactic/Blueprints/Core/Combat/Spells/SpellAnimations/Material/SA_Attack_Interactive/0_BP_Attack_Interactive_ATI.Splash` _attack_interactive false)
      (bind (_direction _over_ro) (`Timeline|OverTimeline` :!via `PlayFromStart` :!label _label_2)
        (:`Update`
          (`/Engine/EditorBlueprintResources/StandardMacros.IsValid` (`self.Attack_Interactive`)
            (:`Is Valid`
              (`self.K2_SetActorTransform` (`self.Attack_Interactive`) (`KismetMathLibrary.MakeTransform` (`SplineComponent.GetLocationAtDistanceAlongSpline` (`self.Spline`) (`SplineComponent.GetSplineLength` (`self.Spline`)) "World") (`KismetMathLibrary.RLerp` Rotator (`self.K2_GetActorRotation` (`/Game/TurnBasedTactic/Blueprints/Core/Combat/Spells/SpellAnimations/Material/SA_Attack_Interactive/0_BP_Attack_Interactive_ATI.Father_Unit` _attack_interactive)) _over_ro true)) false false))))
        (:`Finished`
          (`/Engine/EditorBlueprintResources/StandardMacros.IsValid` (`self.Attack_Interactive`)
            (:`Is Valid`
              (`/Game/TurnBasedTactic/Blueprints/Core/Combat/Spells/SpellAnimations/Material/SA_Attack_Interactive/0_BP_Attack_Interactive_ATI.F_Use_Attack_Range` _attack_interactive_2 true)
              (`/Game/TurnBasedTactic/Blueprints/Core/Combat/Spells/SpellAnimations/Material/SA_Attack_Interactive/0_BP_Attack_Interactive_ATI.Path_Anima_Over` _attack_interactive_2)
              (`self.Path_Clear_Actor`))))))))

(event `Stop_OverTimeline`
  (goto _label_2 :!via `Stop`))

(event `self.Path_Stop_Timeline`
  ;[1 1 1] 停止时间轴动画
  (`self.Stop_BaseTimeLine`)
  (`self.Stop_OverTimeline`)
  (`self.Path_Clear_Actor`))

(fn `UserConstructionScript`
  (`parent.UserConstructionScript`))