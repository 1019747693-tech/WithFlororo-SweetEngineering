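; Spline path actor that flies an attack animation's AttackInteractive aircraft toward a target in the tactics game.
; Construction builds a fixed-angle turning arc toward the target's side, then a straight run, or a closed loop if it circles back, leaving debug arrows and text.
; BaseTimeline moves and banks the aircraft using spline tangents.
; OverTimeline handlers align it to FatherUnit and finish the attack, but PathOverTimeMove is empty and that timeline's play call is unreachable.
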(event `self.Path_Actor_Spline_Mesh_Move`
  (bind _spline (`self.Spline`))
  (bind _attack_interactive (`self.Attack_Interactive`))
  (`TimelineComponent.SetPlayRate` (`self.BaseTimeline`) (/ 1.0 (* (* (`SplineComponent.GetSplineLength` (`self.Spline`)) 0.001) (`self.Anim_Speed`)))) ; 设置动画速率
  (bind (_direction _path_rota_scales) (`Timeline|BaseTimeline` :!via `PlayFromStart` :!label _label)
    (:`Update`
      (`/Engine/EditorBlueprintResources/StandardMacros.IsValid` _attack_interactive
        (:`Is Valid`
          (bind _returnvalue (* (`KismetMathLibrary.Fraction` (.x _path_rota_scales)) (`SplineComponent.GetSplineLength` (`self.Spline`))))
          (bind (_returnvalue_x _returnvalue_y _returnvalue_z) (`KismetMathLibrary.BreakVector` (`KismetMathLibrary.Cross_VectorVector` (`KismetMathLibrary.Normal` (`SplineComponent.GetDirectionAtDistanceAlongSpline` (`self.Spline`) _returnvalue "World")) (`KismetMathLibrary.Normal` (`SplineComponent.GetDirectionAtDistanceAlongSpline` (`self.Spline`) (+ _returnvalue 100.0) "World")))))
          (bind _returnvalue_2 (`SplineComponent.GetRotationAtDistanceAlongSpline` _spline _returnvalue "World"))
          (`self.K2_SetActorTransform` _attack_interactive (`KismetMathLibrary.MakeTransform` (`SplineComponent.GetLocationAtDistanceAlongSpline` _spline _returnvalue "World") (`KismetMathLibrary.ComposeRotators` (`KismetMathLibrary.MakeRotator` (`KismetMathLibrary.Lerp` 0.0 (* _returnvalue_z (* (`self.AC_Angle`) 5.0)) (.y _path_rota_scales))) _returnvalue_2) (`KismetMathLibrary.Conv_DoubleToVector` (.z _path_rota_scales))) false false))))
    (:`Finished`
      (`/Engine/EditorBlueprintResources/StandardMacros.IsValid` (`self.Attack_Interactive`)
        (:`Is Valid`
          (`self.Path_OverTime_Move` _returnvalue_2))
        (:`Is Not Valid`
          (`self.Path_Clear_Actor`))))))

(event `Stop_BaseTimeLine`
  (goto _label :!via `Stop`))

(event `self.Path_OverTime_Move`
  (params (Rotator :type "Rotator Structure")))

(event `Stop_OverTimeline`
  (bind _attack_interactive (`self.Attack_Interactive`))
  (bind (_direction _over_ro) (`Timeline|OverTimeline` :!via `Stop`)
    (:`Update`
      (`/Engine/EditorBlueprintResources/StandardMacros.IsValid` (`self.Attack_Interactive`)
        (:`Is Valid`
          (`self.K2_SetActorTransform` (`self.Attack_Interactive`) (`KismetMathLibrary.MakeTransform` (`SplineComponent.GetLocationAtDistanceAlongSpline` (`self.Spline`) (`SplineComponent.GetSplineLength` (`self.Spline`)) "World") (`KismetMathLibrary.RLerp` (stale `self.Path_OverTime_Move` Rotator) (`self.K2_GetActorRotation` (`/Game/TurnBasedTactic/Blueprints/Core/Combat/Spells/SpellAnimations/Material/SA_Attack_Interactive/0_BP_Attack_Interactive_ATI.Father_Unit` (`self.Attack_Interactive`))) _over_ro true)) false false))))
    (:`Finished`
      (`/Engine/EditorBlueprintResources/StandardMacros.IsValid` (`self.Attack_Interactive`)
        (:`Is Valid`
          (`/Game/TurnBasedTactic/Blueprints/Core/Combat/Spells/SpellAnimations/Material/SA_Attack_Interactive/0_BP_Attack_Interactive_ATI.F_Use_Attack_Range` _attack_interactive true)
          (`/Game/TurnBasedTactic/Blueprints/Core/Combat/Spells/SpellAnimations/Material/SA_Attack_Interactive/0_BP_Attack_Interactive_ATI.Path_Anima_Over` _attack_interactive)
          (`self.Path_Clear_Actor`))))))

(event `self.Path_Stop_Timeline`
  ;[1 1 1] 停止时间轴动画
  (`self.Stop_BaseTimeLine`)
  (`self.Stop_OverTimeline`)
  (`self.Path_Clear_Actor`))

(fn `F_Angle_Between_Points`
  (params (Input_EndPosit :type "Vector Structure") (Input_BeginPosit :type "Vector Structure") (Input_Vector :type "Vector Structure"))
  (returns (Angle_Output :type "Float (double-precision)"))
  (locals (NewLocalVar :type "Float (double-precision)" :default 0.0))
  (return (`KismetMathLibrary.RadiansToDegrees` (`KismetMathLibrary.Acos` (`KismetMathLibrary.Dot_VectorVector` (`KismetMathLibrary.Normal` (- Input_EndPosit Input_BeginPosit)) Input_Vector)))))

(fn `F_Rotated_Target_Location`
  (params (Input_Begin_Position :type "Vector Structure") (Input_Vector :type "Vector Structure") (Base_Rotator :type "Float (double-precision)"))
  (returns (Angle_Position :type "Vector Structure"))
  (return (+ (* (`KismetMathLibrary.GreaterGreater_VectorRotator` (`KismetMathLibrary.Normal` Input_Vector) (`KismetMathLibrary.MakeRotator` 0.0 0.0 (+ Base_Rotator (* (`self.AC_Angle`) (`KismetMathLibrary.SignOfFloat` (`self.Left_Or_Right`)))))) (`self.Point_Distance`)) Input_Begin_Position)))

(fn `F_Set_Base_VectorATT`
  (params (Input_End_Postion :type "Vector Structure"))
  (bind _input_rotator (`self.Input_Rotator`))
  (bind _returnvalue (`KismetMathLibrary.MakeRotator` 0.0 0.0 (`self.Input_Vector`)))
  (bind _returnvalue_2 (`KismetMathLibrary.Normal` (- Input_End_Postion (`self.Begin_Position`))))
  (`SceneComponent.K2_SetWorldRotation` (`self.Arrow`) _returnvalue false false)
  (set `self.Input_Rotator` _returnvalue)
  (set `self.Front_Or_Back` (`KismetMathLibrary.Dot_VectorVector` _returnvalue_2 (`KismetMathLibrary.GetForwardVector` _input_rotator))) ; 确定前后,1为最前最后
  (set `self.Left_Or_Right` (`KismetMathLibrary.Dot_VectorVector` _returnvalue_2 (`KismetMathLibrary.GetRightVector` _input_rotator))) ; 确定左右,1为最左最右
  (set `self.FB_Lerp` (- 1.0 (/ (+ (`self.Front_Or_Back`) 1.0) 2.0))))

(fn `F_Set_Curve_Position`
  (params (F_Over_Position :type "Vector Structure (by ref)"))
  (returns (Spline :type "SplineComponent Object Reference") (`Out_Put_Round?` :type Boolean))
  (locals (Last_Postion :type "Array of Vector Structure") (Lerp :type "Float (double-precision)" :default 0.0) (`Round?` :type Boolean))
  (bind _spline (`self.Spline`))
  (bind _first_position (`self.First_Position`))
  (bind _first_position_2 (`self.First_Position`))
  (bind _first_position_3 (`self.First_Position`))
  (bind _first_position_4 (`self.First_Position`))
  (bind _second_postion (`self.Second_Postion`))
  (bind _first_position_5 (`self.First_Position`))
  (bind _first_position_6 (`self.First_Position`))
  (bind _returnvalue (`KismetArrayLibrary.Array_Length` (`self.First_Position`)))
  (bind _output (`|GetArrayItem` _first_position_6 (- (`KismetArrayLibrary.Array_Length` _first_position_6) 1)))
  (bind _output_2 (`|GetArrayItem` _first_position_4 (- (`KismetArrayLibrary.Array_Length` _first_position_4) 1)))
  (bind _output_3 (`|GetArrayItem` (`self.First_Position`) (- _returnvalue 1)))
  (bind _output_4 (`|GetArrayItem` (`self.First_Position`) (- _returnvalue 2)))
  (bind _returnvalue_2 (`KismetMathLibrary.FindLookAtRotation` _output_3 (`local.F_Over_Position`)))
  (bind _returnvalue_3 (`KismetMathLibrary.FindLookAtRotation` _output_4 _output_3))
  (bind _returnvalue_4 (* (`KismetMathLibrary.SignOfFloat` (`self.Left_Or_Right`)) (`KismetMathLibrary.SignOfFloat` (.z (`KismetMathLibrary.Cross_VectorVector` (`KismetMathLibrary.GetForwardVector` _returnvalue_2) (`KismetMathLibrary.GetForwardVector` _returnvalue_3))))))
  (`KismetArrayLibrary.Array_Clear` _first_position_5)
  (`KismetArrayLibrary.Array_Add` _first_position_5 (`self.Begin_Position`))
  (`KismetArrayLibrary.Array_Clear` (`local.Last_Postion`))
  (`SplineComponent.ClearSplinePoints` (`self.Spline`) true)
  (set `local.Lerp` (`KismetMathLibrary.FClamp` (`KismetMathLibrary.MapRangeClamped` (`self.FB_Lerp`) 0.0 0.2 0.0 1.0)))
  ;[1 1 1] 把新创建点,终点的角度,比上上一个创建点,新创建点的角度,比较目标点是否已经处于轨迹的外环.如果是外环,则不在新创建点,而是以目标向量距离点为准创建新点
  (bind _angle_position (`self.F_Rotated_Target_Location` (`self.Begin_Position`) (`SceneComponent.GetForwardVector` (`self.DefaultSceneRoot`)) (`self.Input_Vector`)))
  (`KismetArrayLibrary.Array_Add` (`self.First_Position`) _angle_position)
  (for _ (range (+ (`KismetMathLibrary.FTrunc` (/ 360.0 (`self.AC_Angle`))) 1))
    (bind _angle_position_2 (`self.F_Rotated_Target_Location` _output_2 (`KismetMathLibrary.Normal` (- _output_3 _output_4))))
    (`AddComponent|NODE_AddArrowComponent-2` :`RelativeTransform` (`KismetMathLibrary.MakeTransform` _output_2 _returnvalue_3 (3.0 3.0 3.0))) ; 每个点朝前的向量
    (`AddComponent|NODE_AddArrowComponent-3` :`RelativeTransform` (`KismetMathLibrary.MakeTransform` _output_2 _returnvalue_2 (3.0 3.0 3.0))) ; 对目标点的向量朝向
    ;;[1 1 1] 检查每个坐标点向量
    (bind _returnvalue_5 (`AddComponent|NODE_AddTextRenderComponent-2` :`RelativeTransform` (`KismetMathLibrary.MakeTransform` _output_2 (struct) (3.0 3.0 3.0))))
    (`TextRenderComponent.K2_SetText` _returnvalue_5 (`|FormatText` "{Z}" _returnvalue_4))
    (if (> _returnvalue_4 0.0)
      (break)
      (else
        (`KismetArrayLibrary.Array_Add` (`self.First_Position`) _angle_position_2)
        (bind _returnvalue_6 (> (`self.Point_Distance`) (`KismetMathLibrary.Vector_Distance` _angle_position_2 (`self.Begin_Position`))))
        (set `local.Round?` _returnvalue_6)
        (if _returnvalue_6
          (break)))))
  (`KismetArrayLibrary.Array_Clear` (`self.Second_Postion`))
  ;[1 1 1] 直线点区间
  (`SplineComponent.SetClosedLoop` (`self.Spline`) (`local.Round?`) true)
  (if (`local.Round?`)
    (`KismetArrayLibrary.Array_Remove` _first_position (- (`KismetArrayLibrary.Array_Length` _first_position) 1))
    (`KismetArrayLibrary.Array_Remove` _first_position)
    (else
      (for _index (range 100)
        (bind _returnvalue_7 (+ (* (`KismetMathLibrary.Normal` (- (`local.F_Over_Position`) _output)) (* (+ _index 1) (`self.Point_Distance`))) _output))
        (if (> (`self.Point_Distance`) (`KismetMathLibrary.Vector_Distance` _returnvalue_7 (`local.F_Over_Position`)))
          (break)
          (else
            (`KismetArrayLibrary.Array_Add` (`self.Second_Postion`) _returnvalue_7))))
      ;[1 1 1] 整理点区间(非环点)
      (`KismetArrayLibrary.Array_Remove` _second_postion (- (`KismetArrayLibrary.Array_Length` _second_postion) 1))
      (`KismetArrayLibrary.Array_Add` (`self.Second_Postion`) (`local.F_Over_Position`))
      (`KismetArrayLibrary.Array_Remove` _first_position_3 (- (`KismetArrayLibrary.Array_Length` _first_position_3) 1))
      (`KismetArrayLibrary.Array_Add` _first_position_3 (/ (+ (`|GetArrayItem` _first_position_2 (- (`KismetArrayLibrary.Array_Length` _first_position_2) 1)) (`|GetArrayItem` (`self.Second_Postion`))) 2.0))))
  (for _array_element (`self.First_Position`)
    (`KismetArrayLibrary.Array_Add` (`local.Last_Postion`) _array_element))
  (for _array_element_2 (`self.Second_Postion`)
    (`KismetArrayLibrary.Array_Add` (`local.Last_Postion`) _array_element_2))
  (for _array_element_3 (`local.Last_Postion`)
    (`SplineComponent.AddSplinePoint` _spline _array_element_3 "World" true))
  (`SplineComponent.AddSplinePointAtIndex` _spline (`self.Begin_Position`) 0 "World" true)
  (return (`self.Spline`) (`local.Round?`)))

(fn `UserConstructionScript`
  (locals (Last_Postion :type "Vector Structure"))
  (bind _end_position (`self.End_Position`))
  (bind _returnvalue (`self.GetTransform` (`self.Attack_Interactive`)))
  (`parent.UserConstructionScript`)
  (`self.K2_SetActorTransform` (`KismetMathLibrary.MakeTransform` (0.0 0.0 0.0)))
  (set `self.Begin_Position` (.location _returnvalue))
  (set `self.Input_Vector` (.yaw (.rotation _returnvalue)))
  (`SplineComponent.ClearSplinePoints` (`self.Spline`) true)
  (`self.F_Set_Base_VectorATT` _end_position)
  (bind _spline (`self.F_Set_Curve_Position` _end_position))
  (if (not true)
    (bind _index_position (`self.F_SetPosit_To_IndexPosit` (`SplineComponent.GetLocationAtDistanceAlongSpline` _spline (`self.AC_Distance`) "Local")))
    (`self.F_Set_Base_VectorATT` _index_position)
    (`self.F_Set_Curve_Position` _index_position))
  (`SceneComponent.K2_SetRelativeLocation` (`self.Arrow`) (`self.Begin_Position`) false false))