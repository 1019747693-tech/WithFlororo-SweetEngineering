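; Naval mine Blueprint for a turn-based tactics game, apparently built on the Attack Interactive (ATI) base, detonating on enemy units, enemy ATIs or other non-friendly hits.
; Construction applies blast-radius scale, collision mesh and idle VFX from data, and sets a range-icon child actor.
; Spawning plays a splash and random path animation from the parent unit.
; Each unit-turn start decrements its age, updating the icon's UI or removing it without exploding at zero.
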(event `self.Event_Touch_ATI`
  (params (`Show?` :type Boolean))
  ;[1 1 1] 鼠标触发显示显示ui
  (if `Show?`
    (`self.F_Reset_Materical`)
    (`SceneComponent.SetVisibility` (`self.Show_Range_Icon`) true false)
    (`self.Event_Jump_UI` (`.Age_Max_17_9DC61480421F64A61B4FB6A981BA59A3` (break `/Game/TurnBasedTactic/Blueprints/Core/Combat/Spells/SpellAnimations/Material/SA_Attack_Interactive/Materical/E_ATI_BaseState` (`.BaseState_9_997CD240407AC492B23DB296C2061696` (break `/Game/TurnBasedTactic/Blueprints/Core/Combat/Spells/SpellAnimations/Material/SA_Attack_Interactive/Materical/E0_ATI_Date` (`self.ATI_Date`))))))))

(event `self.Path_Anima_Over`
  ;[1 1 1] 路径动画结束
  (`self.Event_Jump_UI` (`.Age_Max_17_9DC61480421F64A61B4FB6A981BA59A3` (break `/Game/TurnBasedTactic/Blueprints/Core/Combat/Spells/SpellAnimations/Material/SA_Attack_Interactive/Materical/E_ATI_BaseState` (`.BaseState_9_997CD240407AC492B23DB296C2061696` (break `/Game/TurnBasedTactic/Blueprints/Core/Combat/Spells/SpellAnimations/Material/SA_Attack_Interactive/Materical/E0_ATI_Date` (`self.ATI_Date`))))))
  (set `self.bCanShowSRUI` true))

(event `Event_Jump_UI`
  (params (UI_Age_Current :type Integer))
  ;[1 1 1] 用于水雷蓝图的跳出UI事件
  (if (`self.bCanShowSRUI`)
    (`/Game/TurnBasedTactic/Blueprints/Core/Combat/Spells/SpellAnimations/Material/SA_Attack_Interactive/Naval_Mine/BP_NavalMine_RangeIcon.Jump_UI` (cast `/Game/TurnBasedTactic/Blueprints/Core/Combat/Spells/SpellAnimations/Material/SA_Attack_Interactive/Naval_Mine/BP_NavalMine_RangeIcon` (`ChildActorComponent.ChildActor` (`self.Show_Range_Icon`)) :!pure true) (== (`self.TeamIndex`) 1) UI_Age_Current (`self.IndexColor`))))

(event `self.ReceiveBeginPlay`
  (`parent.ReceiveBeginPlay`)
  (set `self.bCanBoom` true)
  (`self.F_Reset_Materical`))

(event `self.Event_Call_ATI_UnitBegin`
  (bind (_basestate_damage _basestate_age_current) (break `/Game/TurnBasedTactic/Blueprints/Core/Combat/Spells/SpellAnimations/Material/SA_Attack_Interactive/Materical/E_ATI_BaseState` (break `/Game/TurnBasedTactic/Blueprints/Core/Combat/Spells/SpellAnimations/Material/SA_Attack_Interactive/Materical/E0_ATI_Date` (`self.ATI_Date`))))
  ;[0 0 0] Unit回合启动的时候，减少该单位剩余回合数
  (bind _result (`/Engine/EditorBlueprintResources/StandardMacros.DecrementInt` _basestate_age_current)
    (:`  `
      (if (<= _result 0)
        (`self.Boom_Master` false self)
        (else
          (`self.Event_Jump_UI` _result))))))

(event `self.Play_PathAnim`
  (bind _ati_date_attack_interactive_asset (break `/Game/TurnBasedTactic/Blueprints/Core/Combat/Spells/SpellAnimations/Material/SA_Attack_Interactive/Materical/E0_ATI_Date` (`self.ATI_Date`)))
  ;[0 0 0] 播放起始动画
  (bind _output_randompath (`self.F Random Path Anim` (`.Brith_Path_24_218CA4D24229C0D5DD193F81A24900F5` (break `/Game/TurnBasedTactic/Blueprints/Core/Combat/Spells/SpellAnimations/Material/SA_Attack_Interactive/Materical/E_ATI_Assets` _ati_date_attack_interactive_asset))))
  (`|SpawnActorFromClass` "/Game/Effects/VFX/VFX_Blueprint/BP_VFX_Splash.BP_VFX_Splash_C" (`KismetMathLibrary.MakeTransform` (0.0 0.0 0.0)) "Undefined" "MultiplyWithRoot" null (`self.K2_GetActorLocation` self) (struct) null)
  (if (`KismetSystemLibrary.IsValidClass` _output_randompath)
    (bind _returnvalue (`|SpawnActorFromClass` _output_randompath (`KismetMathLibrary.MakeTransform` (0.0 0.0 0.0)) "Undefined" "MultiplyWithRoot" null (`self.K2_GetActorLocation` (`self.Father_Unit`)) (`self.K2_GetActorLocation` self) self (0.0 0.0) null)) ; 播放path动画
    (set `self.ATI_BP_Path` _returnvalue)
    (`self.Event_Touch_ATI` true)))

(event `self.Hurt_Class`
  (params (Actor :type "Actor Object Reference"))
  (bind _ati_bp_path (`self.ATI_BP_Path`))
  ;[1 0 0] 触发水雷爆炸
  (`self.F_Boom_By_NavalMine` Actor)
  (`/Engine/EditorBlueprintResources/StandardMacros.IsValid` _ati_bp_path ; 用于水雷生成后判断路径是否存在
    (:`Is Valid`
      (`self.K2_DestroyActor` _ati_bp_path))))

(fn `F_Boom_By_NavalMine`
  (params (Actor :type "Actor Object Reference"))
  (bind (_as0_bp_unit _bsuccess) (cast `/Game/TurnBasedTactic/Blueprints/Core/Units/0_BP_Unit` Actor :!pure true))
  (bind (_as0_bp_attack_interactive_ati _bsuccess_2) (cast `/Game/TurnBasedTactic/Blueprints/Core/Combat/Spells/SpellAnimations/Material/SA_Attack_Interactive/0_BP_Attack_Interactive_ATI` Actor :!pure true))
  (if _bsuccess
    (if (!= (`/Game/TurnBasedTactic/Blueprints/Core/Units/0_BP_Unit.TeamIndex` _as0_bp_unit) (`self.TeamIndex`))
      (`KismetSystemLibrary.PrintText` "敌" false false)
      (`self.Boom_Master` true _as0_bp_unit)
      (else
        (`KismetSystemLibrary.PrintText` "友" false false)))
    (elif _bsuccess_2
      (if (!= (`self.TeamIndex`) (`/Game/TurnBasedTactic/Blueprints/Core/Combat/Spells/SpellAnimations/Material/SA_Attack_Interactive/0_BP_Attack_Interactive_ATI.TeamIndex` _as0_bp_attack_interactive_ati))
        (`KismetSystemLibrary.PrintText` "ATI_敌" false false)
        (`self.Boom_Master` true)
        (`self.ATI_Boom`)
        (`/Engine/EditorBlueprintResources/StandardMacros.IsValid` _as0_bp_attack_interactive_ati
          (:`Is Valid`
            (`self.Boom_Master` _as0_bp_attack_interactive_ati true null)))
        (else
          (`KismetSystemLibrary.PrintText` "ATI_友" false false)))
      (else
        (`KismetSystemLibrary.PrintText` "墙" false false) ; 啥也没击中就是墙了
        (`self.Boom_Master` true)
        (`self.ATI_Boom`)))))

(fn `Ready_NavalMine`
  (bind _returnvalue_location (`KismetMathLibrary.BreakTransform` (`SceneComponent.GetSocketTransform` (`self.Mesh`) "Attack_Range" "RTS_Actor")))
  (`ChildActorComponent.SetChildActorClass` (`self.Show_Range_Icon`) "/Game/TurnBasedTactic/Blueprints/Core/Combat/Spells/SpellAnimations/Material/SA_Attack_Interactive/Naval_Mine/BP_NavalMine_RangeIcon.BP_NavalMine_RangeIcon_C")
  ;[1 1 1] 爆炸标识缩放
  (`SceneComponent.SetWorldScale3D` (`self.Attack_Range`) (`KismetMathLibrary.Conv_DoubleToVector` (* (`.Blast_Radius_18_E0D57E7D444530BD4D387E9CF00DD2AA` (break `/Game/TurnBasedTactic/Blueprints/Core/Combat/Spells/SpellAnimations/Material/SA_Attack_Interactive/Materical/E_ATI_DateNavalMine` (`self.NavalMine_Date`))) 0.01)))
  ;[1 1 1] 碰撞体模型
  (`StaticMeshComponent.SetStaticMesh` (`self.Attack_Range`) (`.Collision_20_72BAA4F44AAAB1929629B4B325C8D08F` (break `/Game/TurnBasedTactic/Blueprints/Core/Combat/Spells/SpellAnimations/Material/SA_Attack_Interactive/Materical/E_ATI_BaseState` (`.BaseState_9_997CD240407AC492B23DB296C2061696` (break `/Game/TurnBasedTactic/Blueprints/Core/Combat/Spells/SpellAnimations/Material/SA_Attack_Interactive/Materical/E0_ATI_Date` (`self.ATI_Date`))))))
  ;[1 1 1] 设置移动待机粒子
  (`ParticleSystemComponent.SetTemplate` (`self.P_Idle`) (`.VFX_Idle_32_4356D8FA4B86A8213B1EC2A4E7EAE5FE` (break `/Game/TurnBasedTactic/Blueprints/Core/Combat/Spells/SpellAnimations/Material/SA_Attack_Interactive/Materical/E_ATI_DateNavalMine` (`self.NavalMine_Date`))))
  ;[1 1 1] 设置水雷顶部碰撞体以及尾部拖尾粒子位置
  (`SceneComponent.K2_SetRelativeLocation` (`self.Attack_Range`) _returnvalue_location false false))

(fn `UserConstructionScript`
  (`parent.UserConstructionScript`)
  (`self.Ready_NavalMine`))