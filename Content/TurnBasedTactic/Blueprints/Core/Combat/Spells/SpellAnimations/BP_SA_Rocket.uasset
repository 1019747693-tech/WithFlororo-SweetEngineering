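; BP_SA_Rocket is the spell animation for a rocket barrage in the turn-based tactics combat.
; When played, it spawns a configurable number of rockets at once, each on a randomly picked attacked grid tile, so tiles can repeat.
; Each detached rocket receives the caster's team, unit and this animation as references.
; Completion fires after a fixed delay, without waiting on the rockets themselves.
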(event `self.ReceiveBeginPlay`
  (`parent.ReceiveBeginPlay`))

(event `self.Event_PlaySpellAnimation`
  (bind _attackedindex (`/Game/TurnBasedTactic/Blueprints/Core/Combat/BP_CombatSystem.AttackedIndex` (`self.CombatSystem`)))
  (for _ (range 1 (+ (`self.Rocket_Number`) 1))
    (`self.F_Brith_Rocket` (`/Game/TurnBasedTactic/Blueprints/Core/Grid/BP_Grid.GetTileLocationFromGridIndex` (`self.Grid`) (`|GetArrayItem` _attackedindex (`KismetMathLibrary.RandomIntegerInRange` 0 (- (`KismetArrayLibrary.Array_Length` _attackedindex) 1))))))
  (`KismetSystemLibrary.Delay` 20.0)
  (`self.Event_CompleteSpellAnimation`))

(fn `F_Brith_Rocket`
  (params (Brith_Position :type "Vector Structure"))
  (locals (`Use_Debug?` :type Boolean :default true))
  (bind _unit (`self.Unit`))
  (set `local.Use_Debug?` false)
  (bind _returnvalue (`|SpawnActorFromClass` (`self.Rocket_Type`) (`KismetMathLibrary.MakeTransform` Brith_Position) "Undefined" "MultiplyWithRoot" null (`/Game/TurnBasedTactic/Blueprints/Core/Units/0_BP_Unit.TeamIndex` _unit) _unit self null))
  (`KismetSystemLibrary.PrintText` "生成一个火箭弹" (`local.Use_Debug?`) false)
  (`self.K2_DetachFromActor` _returnvalue "KeepRelative" "KeepRelative" "KeepRelative"))

(fn `UserConstructionScript`
  (`parent.UserConstructionScript`))