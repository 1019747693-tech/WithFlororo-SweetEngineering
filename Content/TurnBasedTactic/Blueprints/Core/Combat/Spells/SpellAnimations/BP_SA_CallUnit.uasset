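; BP_SA_CallUnit is a spell animation Blueprint that summons a new unit into combat.
; When played, it prints a debug message and spawns a 0_BP_Unit using the DT_Hude_DataTable unit data.
; It finds BP_PlayerActions and registers the unit with its CombatSystem at the target index, as an AI-controlled member of the caster's team.
; It then signals completion immediately, with no visual effects or delay.
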(event `self.Event_PlaySpellAnimation`
  (bind _unit (`self.Unit`))
  (`KismetSystemLibrary.PrintText` "召唤单位")
  (bind _returnvalue (`|SpawnActorFromClass` "/Game/TurnBasedTactic/Blueprints/Core/Units/0_BP_Unit.0_BP_Unit_C" (`KismetMathLibrary.MakeTransform` (0.0 0.0 0.0)) "Undefined" "MultiplyWithRoot" null 0 "/Game/Character/Char/Hude/DT_Hude_DataTable.DT_Hude_DataTable" null))
  (bind _returnvalue_2 (`GameplayStatics.GetActorOfClass` "/Game/TurnBasedTactic/Blueprints/Core/Player/BP_PlayerActions.BP_PlayerActions_C"))
  (`/Game/TurnBasedTactic/Blueprints/Core/Combat/BP_CombatSystem.AddUnitInCombat` (`/Game/TurnBasedTactic/Blueprints/Core/Player/BP_PlayerActions.CombatSystem` _returnvalue_2) _returnvalue (`self.TargetIndex`) (`/Game/TurnBasedTactic/Blueprints/Core/Units/0_BP_Unit.TeamIndex` _unit) true _unit)
  (`self.Event_CompleteSpellAnimation`))

(fn `UserConstructionScript`
  (`parent.UserConstructionScript`))