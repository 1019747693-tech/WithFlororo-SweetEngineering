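; Spell animation actor for a turn-based tactics game that launches one to three torpedoes at a target tile.
; When played, it builds transforms at that tile, offset sideways along the unit's right vector and yawed 90 degrees from the unit.
; It spawns a BPTorpedo at each, passing team, unit and itself.
; Destroy_By_Torpedo counts finished torpedoes and completes the animation once all are done.
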(event `self.ReceiveBeginPlay`
  (`parent.ReceiveBeginPlay`)
  (set `self.Destroy_By_Torpedo_Number` 0))

(event `self.Event_PlaySpellAnimation`
  (`self.F_Create_Torpedo_Position`))

(event `Destroy_By_Torpedo`
  ;[1 1 1] 计算鱼雷数，到数后销毁自己
  (bind _result (`/Engine/EditorBlueprintResources/StandardMacros.IncrementInt` (`self.Destroy_By_Torpedo_Number`))
    (:`  `
      (if (== _result (`self.Have_Torpedo_Number`))
        (`KismetSystemLibrary.PrintText` "已被销毁" false false)
        (`self.Event_CompleteSpellAnimation`)
        (else
          (`KismetSystemLibrary.PrintText` (`|FormatText` "{A}发鱼雷已被引爆" _result) false false))))))

(fn `F_Create_Torpedo_Position`
  (bind _unit (`self.Unit`))
  (bind _torpedo_postion (`self.Torpedo_Postion`))
  (bind _unit_2 (`self.Unit`))
  (bind _transform_location (`KismetMathLibrary.BreakTransform` (`self.GetTileTransform` (`self.TargetIndex`))))
  (bind (_returnvalue_location _returnvalue_rotation) (`KismetMathLibrary.BreakTransform` (`self.GetTransform` _unit)))
  (bind _returnvalue (* (`KismetMathLibrary.Normal` (`self.GetActorRightVector` _unit)) 200.0))
  (bind _returnvalue_2 (`KismetMathLibrary.MakeRotator` (.roll _returnvalue_rotation) (.pitch _returnvalue_rotation) (+ (.yaw _returnvalue_rotation) 90.0)))
  (bind _returnvalue_3 (`KismetMathLibrary.MakeTransform` (- _transform_location _returnvalue) _returnvalue_2))
  (bind _returnvalue_4 (`KismetMathLibrary.MakeTransform` _transform_location _returnvalue_2))
  (bind _returnvalue_5 (`KismetMathLibrary.MakeTransform` (+ _transform_location _returnvalue) _returnvalue_2))
  (`KismetArrayLibrary.Array_Clear` (`self.Torpedo_Postion`))
  (switch `/Game/TurnBasedTactic/Blueprints/Core/Combat/Spells/SpellAnimations/Material/SA_Attack_Interactive/Torpedo/BaseMatercail/DF_Torpedo_Number` (`self.Torpedo_Number`)
    (:`NewEnumerator0`
      (`KismetArrayLibrary.Array_Add` (`self.Torpedo_Postion`) _returnvalue_4)
      (set `self.Have_Torpedo_Number` 1))
    (:`NewEnumerator1`
      (`KismetArrayLibrary.Array_Add` (`self.Torpedo_Postion`) _returnvalue_5)
      (`KismetArrayLibrary.Array_Add` (`self.Torpedo_Postion`) _returnvalue_3)
      (set `self.Have_Torpedo_Number` 2))
    (:`NewEnumerator2`
      (`KismetArrayLibrary.Array_Add` _torpedo_postion _returnvalue_4)
      (`KismetArrayLibrary.Array_Add` _torpedo_postion _returnvalue_5)
      (`KismetArrayLibrary.Array_Add` _torpedo_postion _returnvalue_3)
      (set `self.Have_Torpedo_Number` 3)))
  (for _array_element (`self.Torpedo_Postion`)
    (`KismetSystemLibrary.PrintText` (`|FormatText` "鱼雷坐标:{A}" (`KismetTextLibrary.Conv_TransformToText` _array_element)))
    (`|SpawnActorFromClass` (`self.BP_Torpedo`) _array_element "Undefined" "MultiplyWithRoot" null (`/Game/TurnBasedTactic/Blueprints/Core/Units/0_BP_Unit.TeamIndex` _unit_2) _unit_2 self null)))

(fn `UserConstructionScript`
  (`parent.UserConstructionScript`))