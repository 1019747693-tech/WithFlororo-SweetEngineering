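; BP_SA_Fire is a spell animation for the turn-based tactics combat system that places a fire actor on the attacked grid tile.
; When played, it converts the first attacked index to a tile location and spawns the configured FireType there, passing team, caster unit and itself.
; It detaches the spawned actor, then signals spell completion after a fixed long delay rather than waiting on that actor.
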(event `self.ReceiveBeginPlay`
  (`parent.ReceiveBeginPlay`))

(event `self.Event_PlaySpellAnimation`
  ;[1 1 1] 开炮
  (`self.F_Brith_Fire` (`/Game/TurnBasedTactic/Blueprints/Core/Grid/BP_Grid.GetTileLocationFromGridIndex` (`self.Grid`) (`|GetArrayItem` (`/Game/TurnBasedTactic/Blueprints/Core/Combat/BP_CombatSystem.AttackedIndex` (`self.CombatSystem`)))))
  (`KismetSystemLibrary.Delay` 20.0)
  (`self.Event_CompleteSpellAnimation`))

(fn `F_Brith_Fire`
  (params (Brith_Position :type "Vector Structure"))
  (locals (`Use_Debug?` :type Boolean :default true))
  (bind _unit (`self.Unit`))
  (set `local.Use_Debug?` false)
  (bind _returnvalue (`|SpawnActorFromClass` (`self.Fire_Type`) (`KismetMathLibrary.MakeTransform` Brith_Position) "Undefined" "MultiplyWithRoot" null (`/Game/TurnBasedTactic/Blueprints/Core/Units/0_BP_Unit.TeamIndex` _unit) _unit self null))
  (`KismetSystemLibrary.PrintText` "发射一发炮弹" (`local.Use_Debug?`) false)
  (`self.K2_DetachFromActor` _returnvalue "KeepRelative" "KeepRelative" "KeepRelative"))

(fn `UserConstructionScript`
  (`parent.UserConstructionScript`))