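; Player action for the overworld that adds or removes units at the cursor.
; When adding, it traces under the cursor, spawns a 0_BP_Unit from the given ID and data, and snaps it to the navigation surface, offset by capsule height.
; The new unit then gets its context set and joins a group through the OverworldUnitGroupsManager.
; When removing, it destroys the currently hovered unit.
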(fn `Execute Action`
  (params (Index :type "IntPoint Structure") (Unit_Anim :type "/Game/TurnBasedTactic/Blueprints/Core/Units/0_BP_Unit Object Reference") (Unit_Date :type "DataTable Object Reference") (UnitID :type Integer))
  (locals (HitLocation :type "Vector Structure") (Unit :type "/Game/TurnBasedTactic/Blueprints/Core/Units/0_BP_Unit Object Reference"))
  (bind _unit (`local.Unit`))
  (bind (_hitresult _returnvalue) (`PlayerController.GetHitResultUnderCursorByChannel` (`GameplayStatics.GetPlayerController` 0) "TraceTypeQuery3" false))
  (bind _hoveredunit (`/Game/TurnBasedTactic/Blueprints/Core/Player/BP_PlayerActions.HoveredUnit` (`self.PlayerActions`)))
  ;[0 0 0] [EN] If we add a unit, make sure the mouse is over the ground, spawn the unit and readjust it on the ground. Otherwise, destroy the unit
  ; [FR] Si on ajoute une unité, on fait sûr que la souris pointe sur le sol, on spawn l'unité et on réajuste sa position pour qu'elle soit sur le sol. Sinon, on fait simplement la détruire
  (if (`self.IsAddingUnit`)
    (if _returnvalue
      (set `local.HitLocation` (`.Location` (`GameplayStatics.BreakHitResult` _hitresult)))
      (bind _returnvalue_2 (`|SpawnActorFromClass` "/Game/TurnBasedTactic/Blueprints/Core/Units/0_BP_Unit.0_BP_Unit_C" (`KismetMathLibrary.MakeTransform` (0.0 0.0 0.0)) "AlwaysSpawn" "MultiplyWithRoot" null (`local.UnitID`) (`local.Unit_Date`) null))
      (set `local.Unit` _returnvalue_2)
      (`self.K2_SetActorLocation` _unit (`/Game/TurnBasedTactic/Blueprints/Core/Units/0_BP_Unit.Add Capsule Height` _unit (`NavigationSystemV1.K2_ProjectPointToNavigation` (`local.HitLocation`) (`/Game/TurnBasedTactic/Blueprints/Core/Units/0_BP_Unit.NavData` _unit) null (500.0 500.0 999999.0))) false false)
      (`/Game/TurnBasedTactic/Blueprints/Core/Units/0_BP_Unit.Set Unit Context` (`local.Unit`) "NewEnumerator1")
      (`/Game/TurnBasedTactic/Blueprints/Core/Units/OverworldUnitGroups/BP_OverworldUnitGroupsManager.AddUnitToGroup` (`/Game/TurnBasedTactic/Blueprints/Core/Player/BP_PlayerActions.OverworldUnitGroupsManager` (`self.PlayerActions`)) (`local.Unit`) (`self.GroupId`)))
    (else
      (`/Engine/EditorBlueprintResources/StandardMacros.IsValid` _hoveredunit
        (:`Is Valid`
          (`self.K2_DestroyActor` _hoveredunit))))))

(fn `UserConstructionScript`
  (`parent.UserConstructionScript`))