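; Player action for the overworld that selects the unit currently under the cursor.
; On execute it looks up the hovered unit's group in the overworld unit groups manager and selects it only if that group is not an encounter.
; Executing with no valid hovered unit clears the selection, as does EndPlay, by passing sentinel tile indices.
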(event `self.ReceiveEndPlay`
  (params (EndPlayReason :type "EEndPlayReason Enum" :default "Destroyed"))
  (`parent.ReceiveEndPlay` EndPlayReason)
  (`/Game/TurnBasedTactic/Blueprints/Core/Player/BP_PlayerActions.Set Selected Tile and Unit` (`self.PlayerActions`) (make `IntPoint` -999 -999) null false))

(fn `Execute Action`
  (params (Index :type "IntPoint Structure") (Unit_Anim :type "/Game/TurnBasedTactic/Blueprints/Core/Units/0_BP_Unit Object Reference") (Unit_Date :type "DataTable Object Reference") (UnitID :type Integer))
  (bind _playeractions (`self.PlayerActions`))
  (bind _playeractions_2 (`self.PlayerActions`))
  ;[0 0 0] [EN] Only select units that are not encounters
  ; [FR] Sélectionne seulement les unités qui ne sont pas encounters
  (`/Engine/EditorBlueprintResources/StandardMacros.IsValid` (`/Game/TurnBasedTactic/Blueprints/Core/Player/BP_PlayerActions.HoveredUnit` (`self.PlayerActions`))
    (:`Is Valid`
      (if (not (`.IsEncounter_8_1C65C7CD455B3EFB2A99CF8347C5BC43` (break `/Game/TurnBasedTactic/Blueprints/Core/Units/OverworldUnitGroups/S_OverworldUnitGroup` (`BlueprintMapLibrary.Map_Find` (`/Game/TurnBasedTactic/Blueprints/Core/Units/OverworldUnitGroups/BP_OverworldUnitGroupsManager.UnitGroups` (`/Game/TurnBasedTactic/Blueprints/Core/Player/BP_PlayerActions.OverworldUnitGroupsManager` _playeractions)) (`/Game/TurnBasedTactic/Blueprints/Core/Units/0_BP_Unit.OverworldGroupId` (`/Game/TurnBasedTactic/Blueprints/Core/Player/BP_PlayerActions.HoveredUnit` _playeractions))))))
        (`/Game/TurnBasedTactic/Blueprints/Core/Player/BP_PlayerActions.Set Selected Tile and Unit` :`self` _playeractions_2 :`Unit` (`/Game/TurnBasedTactic/Blueprints/Core/Player/BP_PlayerActions.HoveredUnit` _playeractions_2))))
    (:`Is Not Valid`
      (`/Game/TurnBasedTactic/Blueprints/Core/Player/BP_PlayerActions.Set Selected Tile and Unit` (`self.PlayerActions`) (make `IntPoint` -999 -999) null false))))

(fn `UserConstructionScript`
  (`parent.UserConstructionScript`))