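; Player action for combat setup that adds a unit to, or removes one from, a grid tile.
; When adding, it checks the tile type against the unit data's valid types, looked up with a fixed ID rather than the passed UnitID.
; It then clears any occupant, spawns the unit and registers it with CombatSystem by team and AI flag.
; Removal reuses the clearing step, which unregisters and destroys the occupant.
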(fn `Execute Action`
  (params (Index :type "IntPoint Structure") (Unit_Anim :type "/Game/TurnBasedTactic/Blueprints/Core/Units/0_BP_Unit Object Reference") (Unit_Date :type "DataTable Object Reference") (UnitID :type Integer))
  (locals (Unit :type "/Game/TurnBasedTactic/Blueprints/Core/Units/0_BP_Unit Object Reference"))
  (bind _unit_date (`self.Unit_Date`))
  ;[0 0 0] [EN] When we add a unit, we first make sure to remove the previous unit (if valid) and then we can spawn the new unit and place it on the grid.
  ; [FR] Quand on ajoute une unité, on fait d'abbord sûr d'enlever l'unité déjà présente sur la case (si valide) et ensuite on peut spawn notre nouvelle unité et la placer sur la grille
  ; [CN] 添加单位时，首先确保移除格子上已有单位（若存在），随后生成新单位并放置到网格。
  (if (`self.IsAddingUnit`)
    ;;[1 1 1] 这里选择添加角色类型
    (bind (_have_unit_ _unit_date_2) (`/Game/TurnBasedTactic/Blueprints/Core/Units/Utilities/BFL_Units.Get Default Unit Data from Unit Type` 1 (`self.Unit_Date`)))
    (if _have_unit_
      (if (`KismetArrayLibrary.Array_Contains` (`.ValidTileTypes_4_6234694045CE2EE6754E4D85BDF64C4A` (break `/Game/TurnBasedTactic/Blueprints/Core/Units/Utilities/S_UnitData_Stats` (`.Stats_10_7052B9524B7C5ED81382818A31190494` (break `/Game/TurnBasedTactic/Blueprints/Core/Units/Utilities/S_UnitData_Test` _unit_date_2)))) (`.Type_5_7348A67046FF7B2ACB404DA293B43DAF` (break `/Game/TurnBasedTactic/Blueprints/Core/Grid/Utilities/S_TileData` (`BlueprintMapLibrary.Map_Find` (`/Game/TurnBasedTactic/Blueprints/Core/Grid/BP_Grid.GridTiles` (`/Game/TurnBasedTactic/Blueprints/Core/Player/BP_PlayerActions.Grid` (`self.PlayerActions`))) (`local.Index`)))))
        (`|ExecutionSequence`
          (:`then_0`
            (bind _output_get (set `local.Unit` (`.UnitOnTile_18_52B829E1479021154B06CAA1E2FD55C2` (break `/Game/TurnBasedTactic/Blueprints/Core/Grid/Utilities/S_TileData` (`BlueprintMapLibrary.Map_Find` (`/Game/TurnBasedTactic/Blueprints/Core/Grid/BP_Grid.GridTiles` (`/Game/TurnBasedTactic/Blueprints/Core/Player/BP_PlayerActions.Grid` (`self.PlayerActions`))) (`local.Index`)))) :!label _label))
            (`/Engine/EditorBlueprintResources/StandardMacros.IsValid` _output_get
              (:`Is Valid`
                (`/Game/TurnBasedTactic/Blueprints/Core/Combat/BP_CombatSystem.RemoveUnitFromCombat` (`/Game/TurnBasedTactic/Blueprints/Core/Player/BP_PlayerActions.CombatSystem` (`self.PlayerActions`)) (`local.Unit`))
                (`self.K2_DestroyActor` (`local.Unit`)))))
          (:`then_1`
            (`KismetSystemLibrary.LogString` (`KismetSystemLibrary.GetObjectName` _unit_date))
            (bind _returnvalue (`|SpawnActorFromClass` "/Game/TurnBasedTactic/Blueprints/Core/Units/0_BP_Unit.0_BP_Unit_C" (`KismetMathLibrary.MakeTransform` (0.0 0.0 0.0)) "AlwaysSpawn" "MultiplyWithRoot" null (`local.UnitID`) _unit_date null))
            (`/Game/TurnBasedTactic/Blueprints/Core/Combat/BP_CombatSystem.AddUnitInCombat` (`/Game/TurnBasedTactic/Blueprints/Core/Player/BP_PlayerActions.CombatSystem` (`self.PlayerActions`)) _returnvalue (`local.Index`) (`self.TeamIndex`) (`self.UseAi`) null)))))
    (else
      (goto _label))))

(fn `UserConstructionScript`
  (`parent.UserConstructionScript`))