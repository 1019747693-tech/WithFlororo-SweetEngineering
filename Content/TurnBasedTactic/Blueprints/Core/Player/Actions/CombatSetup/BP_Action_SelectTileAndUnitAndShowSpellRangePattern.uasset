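; Player action for combat setup that selects a tile and unit, then previews a spell's range and area-of-effect pattern on the grid.
; Executing it runs the parent action, then marks tiles from CombatSystem's GetSpellRange around the selected tile with a range state.
; Hovering refreshes a separate AoE state, drawn only when the hovered tile is in range.
; One particular AoE pattern value marks just the hovered tile.
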(fn `Execute Action`
  (params (Index :type "IntPoint Structure") (Unit_Anim :type "/Game/TurnBasedTactic/Blueprints/Core/Units/0_BP_Unit Object Reference") (Unit_Date :type "DataTable Object Reference") (UnitID :type Integer))
  ;[0 0 0] [EN] Select tile then draw pattern
  ; [FR] Sélectionne la case et ensuite dessine le pattern
  ; [CN] 选择格子后绘制模式
  (`parent.Execute Action` Index Unit_Anim Unit_Date UnitID)
  (`self.ShowSpellRangePattern`))

(fn `ExecuteHoveredAction`
  (params (Index :type "IntPoint Structure"))
  (`parent.ExecuteHoveredAction` Index)
  (`self.ShowSpellRangePatternAoe`))

(fn `ShowSpellRangePattern`
  (bind _playeractions (`self.PlayerActions`))
  (bind _playeractions_2 (`self.PlayerActions`))
  ;[0 0 0] [EN] Clear the previous state and then, if we have a valid index selected, draw the new state on the tiles
  ; [FR] Clear le state précédent et ensuite, si on a un index valide de sélectionné, on dessine le nouveau state sur les cases
  ; [CN] 清除先前状态后，若存在有效选中索引，则在格子上绘制新状态
  (`|ExecutionSequence`
    (:`then_0`
      (`/Game/TurnBasedTactic/Blueprints/Core/Grid/BP_Grid.ClearStateFromTiles` (`/Game/TurnBasedTactic/Blueprints/Core/Player/BP_PlayerActions.Grid` (`self.PlayerActions`)) "NewEnumerator12")
      (if (`/Game/TurnBasedTactic/Blueprints/Core/Grid/BP_Grid.IsIndexValid` (`/Game/TurnBasedTactic/Blueprints/Core/Player/BP_PlayerActions.Grid` _playeractions_2) (`/Game/TurnBasedTactic/Blueprints/Core/Player/BP_PlayerActions.SelectedTile` _playeractions_2))
        (bind _rangeindexes (`/Game/TurnBasedTactic/Blueprints/Core/Combat/BP_CombatSystem.Get Spell Range` (`/Game/TurnBasedTactic/Blueprints/Core/Player/BP_PlayerActions.CombatSystem` _playeractions) (`/Game/TurnBasedTactic/Blueprints/Core/Player/BP_PlayerActions.SelectedTile` _playeractions) (`self.Cast`)))
        (for _array_element _rangeindexes
          (`/Game/TurnBasedTactic/Blueprints/Core/Grid/BP_Grid.AddStateToTile` (`/Game/TurnBasedTactic/Blueprints/Core/Player/BP_PlayerActions.Grid` (`self.PlayerActions`)) _array_element "NewEnumerator12"))))
    (:`then_1`
      (`self.ShowSpellRangePatternAoe`))))

(fn `ShowSpellRangePatternAoe`
  (bind _playeractions (`self.PlayerActions`))
  ;[0 0 0] [EN] Clear the previous state and then, if we have a valid index hovered, draw the new state on the tiles
  ; [FR] Clear le state précédent et ensuite, si on a un index valide sous la souris, on dessine le nouveau state sur les cases
  ; [CN] 清除先前状态后，若存在有效悬停索引，则在格子上绘制新状态
  (`/Game/TurnBasedTactic/Blueprints/Core/Grid/BP_Grid.ClearStateFromTiles` (`/Game/TurnBasedTactic/Blueprints/Core/Player/BP_PlayerActions.Grid` (`self.PlayerActions`)) "NewEnumerator13")
  (if (`KismetArrayLibrary.Array_Contains` (`.IntPointArray_3_F49B81C34A025244B7B55CAC55F1AC35` (break `/Game/TurnBasedTactic/Blueprints/Core/Grid/Utilities/S_IntPointArray` (`BlueprintMapLibrary.Map_Find` (`/Game/TurnBasedTactic/Blueprints/Core/Grid/BP_Grid.TileStateToIndexes` (`/Game/TurnBasedTactic/Blueprints/Core/Player/BP_PlayerActions.Grid` (`self.PlayerActions`))) "NewEnumerator12"))) (`/Game/TurnBasedTactic/Blueprints/Core/Player/BP_PlayerActions.HoveredTile` (`self.PlayerActions`)))
    (if (`|EnumInequality` (`.RangePattern_2_8727DF7A49B477280B09659F1F17B3E5` (break `/Game/TurnBasedTactic/Blueprints/Core/Combat/Spells/Utilities/S_SpellData_Cast` (`self.CastAoe`))) "NewEnumerator0")
      (bind _rangeindexes (`/Game/TurnBasedTactic/Blueprints/Core/Combat/BP_CombatSystem.Get Spell Range` (`/Game/TurnBasedTactic/Blueprints/Core/Player/BP_PlayerActions.CombatSystem` _playeractions) (`/Game/TurnBasedTactic/Blueprints/Core/Player/BP_PlayerActions.HoveredTile` _playeractions) (`self.CastAoe`)))
      (for _array_element _rangeindexes
        (`/Game/TurnBasedTactic/Blueprints/Core/Grid/BP_Grid.AddStateToTile` (`/Game/TurnBasedTactic/Blueprints/Core/Player/BP_PlayerActions.Grid` (`self.PlayerActions`)) _array_element "NewEnumerator13"))
      (else
        (`/Game/TurnBasedTactic/Blueprints/Core/Grid/BP_Grid.AddStateToTile` (`/Game/TurnBasedTactic/Blueprints/Core/Player/BP_PlayerActions.Grid` (`self.PlayerActions`)) (`/Game/TurnBasedTactic/Blueprints/Core/Player/BP_PlayerActions.HoveredTile` (`self.PlayerActions`)) "NewEnumerator13")))))

(fn `UserConstructionScript`
  (`parent.UserConstructionScript`))